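; BP_Button04 is a level-select button that displays a level's name, number and image, and reacts when hit by the player.
; The construction script looks up LevelIndex in DT_LevelList, then fills two text renders and tints them.
; It also sets display color and emissive image through dynamic material instances on the skeletal mesh and image plane.
; HitbyPlayer calls CallHitButton with the level name, plays a sound and animates the button.
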(event EventHitbyPlayer
  (params (HitDirection :type Vector :default "0, 0, 0") (HitLocation :type Vector :default "0, 0, 0") (HitBone :type Name :default "None") (Damage :type Float%20%28single-precision%29) (SpecialDamage :type Special%20Damage%20Struct%20Structure))
  (Default|CallHitButton (Variables|Default|GetLevelName))
  (Audio|PlaySoundatLocation "/Game/Sounds/MenuHit_Cue.MenuHit_Cue" (Transformation|GetActorLocation) "0, 0, 0" 1.0 1.0 0.0 0 0 0)
  (Components|Animation|PlayAnimation (Variables|Default|GetSkeletalMesh) (.OutItem (Utilities|Array|Random (Utilities|Array|MakeArray "/Game/Meshes/Buttons/Animations/Button01_Anim02.Button01_Anim02" "/Game/Meshes/Buttons/Animations/Button01_Anim02.Button01_Anim02"))) false))

(fn ConstructionScript
  (bind _textrender_levelname (Variables|Default|GetTextRender_LevelName))
  (bind _color (Variables|Default|GetColor))
  (bind _levelindex (Variables|Default|GetLevelIndex))
  (bind _returnvalue (Utilities|String|ToString(Integer) _levelindex))
  (CallFunction|CreateMaterialInstancies)
  (CallFunction|GetLevelData)
  (Rendering|Components|TextRender|SetText _textrender_levelname (Utilities|Text|ToText(String) (Utilities|String|Append (Utilities|String|ToString(Text) (Variables|Default|GetDisplayWorldName)) "" " 
" (Utilities|String|ToString(Text) (Variables|Default|GetDisplayLevelName)))))
  (Rendering|Components|TextRender|SetText (Variables|Default|GetTextRender_LevelNumber) (Utilities|Text|ToText(String) (Utilities|String|Append "Level" " " (Utilities|String|SelectString (Utilities|String|Append "0" _returnvalue) _returnvalue (== (Utilities|String|Len _returnvalue) 1)))))
  (Rendering|Components|TextRender|SetTextRenderColor _textrender_levelname (Math|Conversions|ToColor(LinearColor) _color false))
  (Rendering|Material|SetVectorParameterValue (Variables|Default|GetMI_Display) "DisplayColor" _color :!class /Script/Engine.MaterialInstanceDynamic)
  (Rendering|Material|SetTextureParameterValue (Variables|Default|GetMI_Image) "EmissiveMap" (Variables|Default|GetImage)))

(fn CreateMaterialInstancies
  (bind _skeletalmesh (Variables|Default|GetSkeletalMesh))
  (bind _imageplane (Variables|Default|GetImagePlane))
  (bind _returnvalue (Rendering|Material|CreateDynamicMaterialInstance _skeletalmesh 0 (Rendering|Material|GetMaterial _skeletalmesh 0) "None" :!class /Script/Engine.PrimitiveComponent))
  (Variables|Default|SetMI_Display _returnvalue)
  (bind _returnvalue_2 (Rendering|Material|CreateDynamicMaterialInstance _imageplane 0 (Rendering|Material|GetMaterial _imageplane 0) "None" :!class /Script/Engine.PrimitiveComponent))
  (Variables|Default|SetMI_Image _returnvalue_2))

(fn GetLevelData
  (bind _returnvalue (Utilities|GetDataTableRow "/Game/Blueprints/DT_LevelList.DT_LevelList" (Utilities|String|StringToName (Utilities|String|ToString(Integer) (Variables|Default|GetLevelIndex))))
    (:then
      (Variables|Default|SetDisplayWorldName (.displayworldname _returnvalue))
      (Variables|Default|SetDisplayLevelName (.displaylevelname _returnvalue))
      (Variables|Default|SetImage (.levelimage _returnvalue))
      (Variables|Default|SetColor (.displaycolor _returnvalue))
      (Variables|Default|SetLevelName (.levelname _returnvalue)))))