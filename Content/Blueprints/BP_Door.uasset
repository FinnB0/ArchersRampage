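; Door for a VR game that either opens on approach or is sealed by an elemental damage type.
; The construction script creates a dynamic seal material showing the symbol and color for its DamageType.
; Normal doors open once when a VRPawn overlaps the trigger.
; If IsLocked, BeginPlay spawns a matching BP_PadLock and binds to its unlock event; the unlock handler flashes the symbol, darkens the seal, then opens the door.
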(event OnComponentBeginOverlap(OpenTrigger)
  (params (OverlappedComponent :type Primitive%20Component%20Object%20Reference) (OtherActor :type Actor%20Object%20Reference) (OtherComp :type Primitive%20Component%20Object%20Reference) (OtherBodyIndex :type Integer) (bFromSweep :type Boolean) (SweepResult :type Hit%20Result%20Structure%20%28by%20ref%29))
  (Utilities|Casting|CastToVRPawn OtherActor)
  (if (Utilities|Enum|Equal(Enum) (Variables|Default|GetDamageType) "NewEnumerator8")
    (Utilities|FlowControl|DoOnce false
      (:Completed
        (Components|Animation|PlayAnimation (Variables|Default|GetDoor) "/Game/Meshes/Doors/ElevatorDoor/Animations/Elevator_Door_Open.Elevator_Door_Open" false)))))

(event Custom|OpenedLockedDoor
  (bind _mi_doorseal (Variables|Default|GetMI_DoorSeal))
  (Rendering|Material|SetVectorParameterValue (Variables|Default|GetMI_DoorSeal) "SymbolColor" (Utilities|Select :Index (Variables|Default|GetDamageType) :NewEnumerator8 "(R=1.000000,G=1.000000,B=1.000000,A=1.000000)" :NewEnumerator0 "(R=1.000000,G=0.000000,B=0.000000,A=1.000000)" :NewEnumerator1 "(R=0.000000,G=0.329412,B=1.000000,A=1.000000)" :NewEnumerator2 "(R=0.533333,G=1.000000,B=0.000000,A=1.000000)" :NewEnumerator3 "(R=1.000000,G=1.000000,B=0.100000,A=1.000000)" :NewEnumerator4 "(R=0.725490,G=0.000000,B=1.000000,A=1.000000)" :NewEnumerator5 "(R=1.000000,G=0.505882,B=0.000000,A=1.000000)" :NewEnumerator6 "(R=0.000000,G=0.960784,B=1.000000,A=1.000000)" :NewEnumerator7 "(R=1.000000,G=0.000000,B=0.792157,A=1.000000)") :!class /Script/Engine.MaterialInstanceDynamic)
  (Utilities|FlowControl|Delay 1.0)
  (Rendering|Material|SetVectorParameterValue _mi_doorseal "SymbolColor" "(R=0.000000,G=0.000000,B=0.000000,A=1.000000)" :!class /Script/Engine.MaterialInstanceDynamic)
  (Rendering|Material|SetVectorParameterValue :self _mi_doorseal :ParameterName "EmissiveColor" :!class /Script/Engine.MaterialInstanceDynamic)
  (Components|Animation|PlayAnimation (Variables|Default|GetDoor) "/Game/Meshes/Doors/ElevatorDoor/Animations/Elevator_Door_Open.Elevator_Door_Open" false))

(event EventBeginPlay
  (if (Variables|Default|GetbIsLocked?)
    (bind _returnvalue (Game|SpawnActorfromClass "/Game/Blueprints/BP_PadLock.BP_PadLock_C" (Transformation|GetWorldTransform (Variables|Default|GetPadlockSocket)) "Undefined" 0 (Variables|Default|GetDamageType) 0))
    (EventDispatchers|BindEventtoLockOpened _returnvalue (EventDispatchers|CreateEvent :!event Custom|OpenedLockedDoor))))

(fn ConstructionScript
  (bind _damagetype (Variables|Default|GetDamageType))
  (bind _mi_doorseal (Variables|Default|GetMI_DoorSeal))
  (bind _returnvalue (Utilities|Select :Index _damagetype :NewEnumerator8 "(R=0.000000,G=0.000000,B=0.000000,A=1.000000)" :NewEnumerator0 "(R=1.000000,G=0.000000,B=0.000000,A=1.000000)" :NewEnumerator1 "(R=0.000000,G=0.329412,B=1.000000,A=1.000000)" :NewEnumerator2 "(R=0.533333,G=1.000000,B=0.000000,A=1.000000)" :NewEnumerator3 "(R=1.000000,G=1.000000,B=0.100000,A=1.000000)" :NewEnumerator4 "(R=0.725490,G=0.000000,B=1.000000,A=1.000000)" :NewEnumerator5 "(R=1.000000,G=0.505882,B=0.000000,A=1.000000)" :NewEnumerator6 "(R=0.000000,G=0.960784,B=1.000000,A=1.000000)" :NewEnumerator7 "(R=1.000000,G=0.000000,B=0.792157,A=1.000000)"))
  (CallFunction|CreateDynamicMaterialInstance)
  (Rendering|Material|SetTextureParameterValue _mi_doorseal "Symbol" (Utilities|Select :Index _damagetype :NewEnumerator8 "/Game/Textures/Template/T_Black.T_Black" :NewEnumerator0 "/Game/Textures/MagicSymbols/T_SymbolFire_A.T_SymbolFire_A" :NewEnumerator1 "/Game/Textures/MagicSymbols/T_SymbolIce_A.T_SymbolIce_A" :NewEnumerator2 "/Game/Textures/MagicSymbols/T_SymbolPoison_A.T_SymbolPoison_A" :NewEnumerator3 "/Game/Textures/MagicSymbols/T_SymbolElectricity_A.T_SymbolElectricity_A" :NewEnumerator4 "/Game/Textures/MagicSymbols/T_SymbolGravity_A.T_SymbolGravity_A" :NewEnumerator5 "/Game/Textures/MagicSymbols/T_SymbolExplosion_A.T_SymbolExplosion_A" :NewEnumerator6 "/Game/Textures/MagicSymbols/T_SymbolLuck_A.T_SymbolLuck_A" :NewEnumerator7 "/Game/Textures/MagicSymbols/T_SymbolSuck_A.T_SymbolSuck_A"))
  (Rendering|Material|SetVectorParameterValue _mi_doorseal "EmissiveColor" _returnvalue :!class /Script/Engine.MaterialInstanceDynamic)
  (Rendering|Material|SetVectorParameterValue _mi_doorseal "DisplayColor" _returnvalue :!class /Script/Engine.MaterialInstanceDynamic))

(fn CreateDynamicMaterialInstance
  (bind _door (Variables|Default|GetDoor))
  (bind _returnvalue (Rendering|Material|CreateDynamicMaterialInstance _door 1 (Rendering|Material|GetMaterial _door 1) "None" :!class /Script/Engine.PrimitiveComponent))
  (Variables|Default|SetMI_DoorSeal _returnvalue))