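; Game instance for a spell-shooting game, handling leaderboards, PlayFab accounts, streamed levels and menus, and pause state.
; Init fetches Epic leaderboards indexed by damage type; SubmitToAllSpells increments a player's score, using a DoOnce gate and delayed refresh.
; LoadLevel and LoadMenu swap streamed levels, with level loads also setting game state and start time.
; PlayFab events register, log in and send stats through CloudScript, but their test sequence is disconnected.
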(event Custom|SubmitToAllSpells
  (params (EntryName :type String) (DamageTypeIndex :type Integer))
  (Utilities|FlowControl|DoOnce false :!label _label
    (:Completed
      (bind _output_get (Variables|Default|SetLeaderboardAllSpells (Utilities|Array|Get(acopy) (Variables|Default|GetAllSpellLeaderboards) DamageTypeIndex)))
      (Utilities|IsValid _output_get
        (:Is%20Valid
          (for _array_element (Variables|/Script/EpicLeaderboard.EpicLeaderboardObject|GetLeaderboardEntries (Variables|Default|GetLeaderboardAllSpells))
            (if (Utilities|Enum|Equal(Enum) (.username (Utilities|Struct|BreakEpicLeaderboardEntry _array_element)) EntryName)
              (Class|EpicLeaderboardObject|SubmitEntry (Variables|Default|GetLeaderboardAllSpells) EntryName (+ (Math|Conversions|ToFloat(Integer) (.score (Utilities|Struct|BreakEpicLeaderboardEntry _array_element))) 1.0))
              (Variables|Default|SetFoundSpell true)))
          (if (Variables|Default|GetFoundSpell)
            _
            (else
              (Class|EpicLeaderboardObject|SubmitEntry (Variables|Default|GetLeaderboardAllSpells) EntryName 1.0)))
          (Utilities|FlowControl|RetriggerableDelay 2.0)
          (Variables|Default|SetFoundSpell false)
          (Class|EpicLeaderboardObject|GetLeaderboardEntries (Variables|Default|GetLeaderboardAllSpells) "" false)
          (goto _label Reset))))))

(event Custom|LoadLevel
  (params (LevelName :type Name) (GameState :type GameState%20Enum :default "NewEnumerator0"))
  (Variables|Default|SetCurrentGameState GameState)
  (if (Utilities|Name|NotEqual(Name) (Variables|Default|GetCurrentLevel) "None")
    (Game|UnloadStreamLevel(byName) (Variables|Default|GetCurrentLevel) false))
  (Game|LoadStreamLevel(byName) LevelName true)
  (Variables|Default|SetCurrentLevel LevelName)
  (Class|BPICameraFade|Fadein(Message) (Game|Player|GetPlayerPawn 0))
  (bind _asgs_spell_shot (Utilities|Casting|CastToGS_SpellShot (Game|GetGameState)))
  (Default|SetLevelStartTime _asgs_spell_shot))

(event Custom|RegisterSuccess
  (params (result :type Client%20Register%20Play%20Fab%20User%20Result%20Structure) (customData :type Object%20Object%20Reference))
  ;[0.3149 1 0.2686 1 30] PlayFab Solution
  ;;[1 1 1] Register to PlayFab
  (CallFunction|UserLoggedin (Utilities|Struct|BreakClientRegisterPlayFabUserResult result)))

(event Custom|RegisterFailed
  (params (error :type Play%20Fab%20Error%20Structure) (customData :type Object%20Object%20Reference))
  ;[0.3149 1 0.2686 1 30] PlayFab Solution
  ;;[1 1 1] Register to PlayFab
  (CallFunction|PrintErrorMessages error))

(event Custom|LogInSuccess
  (params (result :type Client%20Login%20Result%20Structure) (customData :type Object%20Object%20Reference))
  ;[0.3149 1 0.2686 1 30] PlayFab Solution
  ;;[1 1 1] LogIn to PlayFab
  (CallFunction|UserLoggedin (Utilities|Struct|BreakClientLoginResult result)))

(event Custom|UpdatePlayerDataOnPLayFab
  (params (Shots :type Integer) (Jumps :type Integer))
  ;[0.3149 1 0.2686 1 30] PlayFab Solution
  ;;[1 1 1] Set Data on PlayFab
  (Variables|Default|SetJsonObject (Class|PlayFabJsonObject|ConstructJsonObject))
  (Class|PlayFabJsonObject|SetField (Variables|Default|GetJsonObject) "Shots" (Class|PlayFabJsonValue|ConstructJsonValueString (Utilities|String|ToString(Integer) Shots)))
  (Class|PlayFabJsonObject|SetField (Variables|Default|GetJsonObject) "Jumps" (Class|PlayFabJsonValue|ConstructJsonValueString (Utilities|String|ToString(Integer) Jumps)))
  (|ExecuteCloudScript (Utilities|Struct|MakeClientExecuteCloudScriptRequest 0 "UpdatePlayerData" (Variables|Default|GetJsonObject)) (delegate Custom|SetDataSuccess) (delegate Custom|SetDataFailed)))

(event Custom|SetDataSuccess
  (params (result :type Client%20Execute%20Cloud%20Script%20Result%20Structure) (customData :type Object%20Object%20Reference))
  ;[0.3149 1 0.2686 1 30] PlayFab Solution
  ;;[1 1 1] Set Data on PlayFab
  (Development|PrintString "Hello"))

(event Custom|SetDataFailed
  (params (error :type Play%20Fab%20Error%20Structure) (customData :type Object%20Object%20Reference))
  ;[0.3149 1 0.2686 1 30] PlayFab Solution
  ;;[1 1 1] Set Data on PlayFab
  (CallFunction|PrintErrorMessages error))

(event Custom|LogInPlayFab
  (params (Password :type String) (Username :type String))
  ;[0.3149 1 0.2686 1 30] PlayFab Solution
  ;;[1 1 1] LogIn to PlayFab
  (|LoginwithPlayFab (Utilities|Struct|MakeClientLoginWithPlayFabRequest 0 0 Password Username) (delegate Custom|LogInSuccess) (delegate Custom|LogInFailed)))

(event Custom|LoadMenu
  (params (MenuName :type Name) (bJustUnload :type Boolean))
  (if (Utilities|Name|NotEqual(Name) (Variables|Default|GetCurrentMenu) "None")
    (Game|UnloadStreamLevel(byName) (Variables|Default|GetCurrentMenu) true))
  (if bJustUnload
    (Variables|Default|SetCurrentMenu "None")
    (else
      (Game|LoadStreamLevel(byName) MenuName true true)
      (Variables|Default|SetCurrentMenu MenuName))))

(event Custom|Unpause
  (Variables|Default|SetCurrentGameState (Variables|Default|GetLastGameState)))

(event Custom|Pause
  (Variables|Default|SetLastGameState (Variables|Default|GetCurrentGameState))
  (Variables|Default|SetCurrentGameState "NewEnumerator2"))

(event Custom|LogInFailed
  (params (error :type Play%20Fab%20Error%20Structure) (customData :type Object%20Object%20Reference))
  ;[0.3149 1 0.2686 1 30] PlayFab Solution
  ;;[1 1 1] LogIn to PlayFab
  (CallFunction|PrintErrorMessages error))

(event Custom|UserLoggedIn
  (params (UserID :type String))
  ;[0.3149 1 0.2686 1 30] PlayFab Solution
  ;;[1 1 1] On Sucessfully LoggingIn to PlayFab
  (bind _output_get (Variables|Default|SetUserID UserID))
  (Development|PrintString _output_get))

(event Custom|RegisterPlayFab
  (params (Display%20Name :type String) (Email :type String) (Password :type String) (Username :type String))
  ;[0.3149 1 0.2686 1 30] PlayFab Solution
  ;;[1 1 1] Register to PlayFab
  (|RegisterPlayFabUser (Utilities|Struct|MakeClientRegisterPlayFabUserRequest Display%20Name Email Password Username) (delegate Custom|RegisterSuccess) (delegate Custom|RegisterFailed)))

(event EventInit
  ;[1 1 1] Get All Leaderboards on Init
  ;;[1 1 1] All (For Errors)
  (bind _returnvalue (Class|EpicLeaderboardObject|GetEpicLeaderboard "716b6fc8788b92f422209e3e588d5b8b" "b3b8041dec"))
  (Utilities|Array|Insert (Variables|Default|GetAllSpellLeaderboards) _returnvalue)
  ;;[1 1 1] Gravity
  (bind _returnvalue_2 (Class|EpicLeaderboardObject|GetEpicLeaderboard "5e744ba2d5935ecba68375f3980ad38b" "e503607e28"))
  (Utilities|Array|Insert (Variables|Default|GetAllSpellLeaderboards) _returnvalue_2 1)
  ;;[1 1 1] Suck
  (bind _returnvalue_3 (Class|EpicLeaderboardObject|GetEpicLeaderboard "9cdcef1800bfbe0194d0639607810bf6" "9cd30e12ab"))
  (Utilities|Array|Insert (Variables|Default|GetAllSpellLeaderboards) _returnvalue_3 2)
  ;;[1 1 1] Fire
  (bind _returnvalue_4 (Class|EpicLeaderboardObject|GetEpicLeaderboard "ba57043dbbf1744ee8fb786e86d901cf" "8927879adb"))
  (Utilities|Array|Insert (Variables|Default|GetAllSpellLeaderboards) _returnvalue_4 3)
  ;;[1 1 1] Explosion
  (bind _returnvalue_5 (Class|EpicLeaderboardObject|GetEpicLeaderboard "a2a8810dc616633d72b90da2271ada78" "d309a8642c"))
  (Utilities|Array|Insert (Variables|Default|GetAllSpellLeaderboards) _returnvalue_5 4)
  ;;[1 1 1] Poison
  (bind _returnvalue_6 (Class|EpicLeaderboardObject|GetEpicLeaderboard "80f559cf89ee3005a5ef51c83da985fc" "e95d7b9d90"))
  (Utilities|Array|Insert (Variables|Default|GetAllSpellLeaderboards) _returnvalue_6 5)
  ;;[1 1 1] Fire
  (bind _returnvalue_7 (Class|EpicLeaderboardObject|GetEpicLeaderboard "f71492d29f6b68754619715b30333a5c" "83ba547322"))
  (Utilities|Array|Insert (Variables|Default|GetAllSpellLeaderboards) _returnvalue_7 6)
  ;;[1 1 1] Electricity
  (bind _returnvalue_8 (Class|EpicLeaderboardObject|GetEpicLeaderboard "a6c84f516c7572323d7eca8ce1ee9b64" "c2160d6270"))
  (Utilities|Array|Insert (Variables|Default|GetAllSpellLeaderboards) _returnvalue_8 7)
  ;;[1 1 1] Electricity
  (bind _returnvalue_9 (Class|EpicLeaderboardObject|GetEpicLeaderboard "98249a77683025bfcc29949cfb9108cb" "201a90488b"))
  (Utilities|Array|Insert (Variables|Default|GetAllSpellLeaderboards) _returnvalue_9 8)
  ;;[1 1 1] Questions
  (bind _returnvalue_10 (Class|EpicLeaderboardObject|GetEpicLeaderboard "897af98348c7faf7b0fea43361e4d60a" "c371fe8ecb"))
  (Utilities|Array|Insert (Variables|Default|GetAllSpellLeaderboards) _returnvalue_10 9)
  (for _array_element (Variables|Default|GetAllSpellLeaderboards)
    (Class|EpicLeaderboardObject|GetLeaderboardEntries _array_element "" false)))

(fn PrintErrorMessages
  (params (PlayFabError :type Play%20Fab%20Error%20Structure%20%28by%20ref%29))
  (bind (_errorname _errormessage _errordetails) (Utilities|Struct|BreakPlayFabError PlayFabError))
  (Development|PrintString _errorname true true "(R=1.000000,G=0.000000,B=0.000000,A=1.000000)")
  (Development|PrintString _errormessage true true "(R=1.000000,G=0.000000,B=0.000000,A=1.000000)")
  (Development|PrintString _errordetails true true "(R=1.000000,G=0.000000,B=0.000000,A=1.000000)"))