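; A static VR teleport destination actor that moves the player's VRPawn to its own location when hit by the player.
; The hit event then tells every connected enemy spawner to spawn an enemy, so arriving at the point triggers its encounter.
; Pause and Unpause events toggle the actor's collision off and on.
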(event Custom|SpawnEnemys
  (bind _connectedenemyspawners (Variables|Default|GetConnectedEnemySpawners))
  (if (Utilities|Array|IsValidIndex _connectedenemyspawners)
    (for _array_element _connectedenemyspawners
      (Default|SpawnEnemy _array_element))))

(event EventHitbyPlayer
  (params (HitDirection :type Vector :default "0, 0, 0") (HitLocation :type Vector :default "0, 0, 0") (HitBone :type Name :default "None") (Damage :type Float%20%28single-precision%29) (SpecialDamage :type Special%20Damage%20Struct%20Structure))
  (Default|Teleport (.AsVRPawn (Utilities|Casting|CastToVRPawn (Game|Player|GetPlayerPawn 0))) (Transformation|GetActorLocation))
  (CallFunction|SpawnEnemys))

(event EventPause
  (Collision|SetActorEnableCollision false))

(event EventUnpause
  (Collision|SetActorEnableCollision true))

(fn ConstructionScript)