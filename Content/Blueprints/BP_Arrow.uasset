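; Arrow actor that builds a four-digit magic spell code from overlaps with numbered BP_Arrow colliders, recoloring its Niagara ribbon per digit.
; A completed code is looked up in DT_MagicSpells: a match plays a sound and locks input, a miss clears it.
; Tick counter-rotates ColliderHolder against actor roll while input is open.
; Reset, hide and show events manage spell state, visibility and ticking.
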(event OnComponentBeginOverlap(MagicCollider)
  (params (OverlappedComponent :type Primitive%20Component%20Object%20Reference) (OtherActor :type Actor%20Object%20Reference) (OtherComp :type Primitive%20Component%20Object%20Reference) (OtherBodyIndex :type Integer) (bFromSweep :type Boolean) (SweepResult :type Hit%20Result%20Structure%20%28by%20ref%29))
  (bind _componenttags (Variables|/Script/Engine.ActorComponent|GetComponentTags OtherComp))
  (bind _output (Utilities|Array|Get(acopy) _componenttags))
  (bind _returnvalue (Utilities|String|ToString(Name) _output))
  (Utilities|Casting|CastToBP_Arrow OtherActor)
  (if (Variables|Default|GetbIsNormal)
    (Utilities|FlowControl|Sequence
      (:then_0
        (bind _output_get (Variables|Default|SetMagicSpellString (Utilities|String|Append (Variables|Default|GetMagicSpellString) _returnvalue)))
        (if (== (Utilities|String|Len _output_get) 4)
          (Variables|Default|SetbIsNormal false)
          (Actor|Tick|SetActorTickEnabled false)
          (Utilities|GetDataTableRow "/Game/Blueprints/DT_MagicSpells.DT_MagicSpells" (Utilities|String|StringToName (Variables|Default|GetMagicSpellString))
            (:then
              (Variables|Default|SetbIsNormal false)
              (Audio|PlaySoundatLocation "/Game/Sounds/MagicSpell_Cue.MagicSpell_Cue" (Transformation|GetActorLocation) "0, 0, 0" 1.0 1.0 0.0 0 0 0)
              (Actor|Tick|SetActorTickEnabled false))
            (:RowNotFound
              (Variables|Default|SetMagicSpellString "")
              (Variables|Default|SetbIsNormal true)
              (CallFunction|SetRibbonColor "(R=1.000000,G=1.000000,B=1.000000,A=1.000000)")
              (Actor|Tick|SetActorTickEnabled true)))))
      (:then_1
        (switch int (- (Math|Conversions|ToInteger(Byte) _returnvalue) 1)
          (:0
            (CallFunction|SetRibbonColor "(R=0.482639,G=0.000000,B=1.000000,A=1.000000)"))
          (:1
            (CallFunction|SetRibbonColor "(R=1.000000,G=0.000000,B=0.586246,A=1.000000)"))
          (:2
            (CallFunction|SetRibbonColor "(R=1.000000,G=0.007519,B=0.000000,A=1.000000)"))
          (:3
            (CallFunction|SetRibbonColor "(R=1.000000,G=0.505721,B=0.000000,A=1.000000)"))
          (:4
            (CallFunction|SetRibbonColor "(R=0.533577,G=1.000000,B=0.000000,A=1.000000)"))
          (:5
            (CallFunction|SetRibbonColor "(R=0.000000,G=1.000000,B=0.365573,A=1.000000)"))
          (:6
            (CallFunction|SetRibbonColor "(R=0.000000,G=0.960508,B=1.000000,A=1.000000)"))
          (:7
            (CallFunction|SetRibbonColor "(R=0.000000,G=0.328579,B=1.000000,A=1.000000)")))))))

(event Custom|HideArrow
  (Rendering|SetActorHiddenInGame true)
  (Actor|Tick|SetActorTickEnabled false))

(event Custom|ShowArrow
  (Rendering|SetActorHiddenInGame false)
  (if (Variables|Default|GetbIsNormal)
    (Actor|Tick|SetActorTickEnabled true)))

(event Custom|ResetArrow
  (Utilities|FlowControl|Delay 0.5)
  (Variables|Default|SetMagicSpellString "")
  (Variables|Default|SetbIsNormal true)
  (CallFunction|SetRibbonColor "(R=1.000000,G=1.000000,B=1.000000,A=1.000000)")
  (Actor|Tick|SetActorTickEnabled true))

(event EventTick
  (params (DeltaSeconds :type Float%20%28single-precision%29))
  (Transformation|SetRelativeRotation (Variables|Default|GetColliderHolder) (Math|Rotator|MakeRotator (* (.roll (Transformation|GetActorRotation)) -1.0) 0.0 0.0) false false))

(fn ConstructionScript)

(fn SetRibbonColor
  (params (Color :type Linear%20Color%20Structure))
  (Niagara|SetNiagaraVariable(LinearColor) (Variables|Default|GetNiagara) "User.RibbonColor" Color))