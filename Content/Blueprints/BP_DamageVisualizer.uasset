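; BP_DamageVisualizer is a short-lived floating damage number that shows a Damage value as world-space text.
; The construction script gives its ProjectileMovement a velocity with random X and Y and a fixed upward Z, so each number drifts differently.
; On BeginPlay it turns the TextRender toward the player camera once, sets the text, and destroys itself after a one-second delay.
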(event EventBeginPlay
  (Transformation|SetWorldRotation (Variables|Default|GetTextRender) (Math|Rotator|FindLookatRotation (Transformation|GetActorLocation) (Camera|GetCameraLocation (Game|GetPlayerCameraManager 0))) false false)
  (Rendering|Components|TextRender|SetText (Variables|Default|GetTextRender) (Utilities|Text|ToText(Integer) (Variables|Default|GetDamage)))
  (Utilities|FlowControl|Delay 1.0)
  (Actor|DestroyActor))

(fn ConstructionScript
  (Variables|/Script/Engine.MovementComponent|SetVelocity (Variables|Default|GetProjectileMovement) (Math|Vector|MakeVector (Math|Random|RandomFloat) (Math|Random|RandomFloat) 1.0)))