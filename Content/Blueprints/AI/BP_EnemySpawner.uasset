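; Enemy spawner actor that places enemies already alerted to the player.
; SpawnEnemy uses up one unit of EnemyAmount, while any remain, to spawn EnemyToSpawn at the spawner's transform.
; A spawned BP_Enemy has LosesFocus turned off and SeePlayer forced on.
; AutoSpawn triggers a single spawn on BeginPlay; further spawns require additional SpawnEnemy calls.
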(event Custom|SpawnEnemy
  (if (> (Variables|Default|GetEnemyAmount) 0)
    (Math|Integer|DecrementInt (Variables|Default|GetEnemyAmount)
      (:%20%20
        (bind _returnvalue (Game|SpawnActorfromClass (Variables|Default|GetEnemyToSpawn) (Transformation|GetActorTransform) "Undefined" self 0))
        (bind _asbp_enemy (Utilities|Casting|CastToBP_Enemy _returnvalue))
        (Variables|/Game/Blueprints/AI/Pawns/BP_Enemy.BP_Enemy_C|SetbLosesFocus _asbp_enemy false)
        (Default|SeePlayer _asbp_enemy true)))))

(event EventBeginPlay
  (if (Variables|Default|GetbAutoSpawn)
    (CallFunction|SpawnEnemy)))

(fn ConstructionScript)