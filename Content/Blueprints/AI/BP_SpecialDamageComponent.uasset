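; Scene component that gives its owner elemental hit reactions, attached to a skeletal or static mesh whose dynamic materials pulse in the damage type's color.
; Non-immune hits route by type: Fire and Electricity tick damage, Ice nearly freezes the owner, Gravity repeatedly pulls it toward the hit and blocks blackboard movement.
; Looping timers and retriggerable delays time effects; immune hits spawn "IMMUN!" text.
; Freeze and pause factors multiply into CustomTimeDilation, with pause also disabling collision.
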(event Custom|ForceOverTime
  (params (SpecialDamageStruct :type Special%20Damage%20Struct%20Structure) (HitLocation :type Vector))
  (Utilities|Time|PauseTimerbyHandle (Variables|Default|GetForceTimer))
  (Variables|Default|SetDamageType (.type SpecialDamageStruct))
  (Variables|Default|SetDamage (.damage SpecialDamageStruct))
  (bind _output_get (Variables|Default|SetDamageSpeed (.tick SpecialDamageStruct)))
  (Variables|Default|SetHit%20Location HitLocation)
  (bind _returnvalue (Utilities|Time|SetTimerbyEvent (EventDispatchers|CreateEvent :!event ForceTick) _output_get true 0.0 (* _output_get -0.99)))
  (Variables|Default|SetForceTimer _returnvalue)
  (CallFunction|SetBlackboardCanMove false)
  (Utilities|FlowControl|RetriggerableDelay (.duration SpecialDamageStruct))
  (Utilities|Time|PauseTimerbyHandle (Variables|Default|GetForceTimer))
  (CallFunction|ResetMaterials)
  (CallFunction|SetBlackboardCanMove true))

(event Custom|ApplySpecialDamage
  (params (SpecialDamageStruct :type Special%20Damage%20Struct%20Structure) (HitLocation :type Vector))
  (bind _type (Utilities|Struct|BreakSpecialDamageStruct SpecialDamageStruct))
  (if (not (Utilities|Array|ContainsItem (Variables|Default|GetDamageImmunity) _type))
    (switch Utilities|FlowControl|Switch|SwitchonDamageType _type
      (:NewEnumerator0
        (CallFunction|DamageOverTime SpecialDamageStruct))
      (:NewEnumerator1
        (CallFunction|FreezeTime SpecialDamageStruct))
      (:NewEnumerator3
        (CallFunction|DamageOverTime SpecialDamageStruct))
      (:NewEnumerator4
        (CallFunction|ForceOverTime SpecialDamageStruct HitLocation)))
    (else
      (Game|SpawnActorfromClass "/Game/Blueprints/BP_DamageVisualizer.BP_DamageVisualizer_C" (Math|Transform|MakeTransform (+ (Transformation|GetActorLocation (Components|GetOwner)) "0, 0,50.000000") "0, 0, 0" "1,1,1") "AlwaysSpawn" 0 (Utilities|Text|MakeLiteralText "IMMUN!") (Utilities|Struct|MakeSlateColor "(R=1.000000,G=0.000000,B=0.000000,A=1.000000)") 0.5 0))))

(event Custom|DamageOverTime
  (params (SpecialDamageStruct :type Special%20Damage%20Struct%20Structure))
  (Utilities|Time|PauseTimerbyHandle (Variables|Default|GetDamageTimer))
  (Variables|Default|SetDamageType (.type SpecialDamageStruct))
  (Variables|Default|SetDamage (.damage SpecialDamageStruct))
  (bind _output_get (Variables|Default|SetDamageSpeed (.tick SpecialDamageStruct)))
  (bind _returnvalue (Utilities|Time|SetTimerbyEvent (EventDispatchers|CreateEvent :!event DamageTick) _output_get true (* _output_get -0.99)))
  (Variables|Default|SetDamageTimer _returnvalue)
  (Utilities|FlowControl|RetriggerableDelay (.duration SpecialDamageStruct))
  (Utilities|Time|PauseTimerbyHandle (Variables|Default|GetDamageTimer))
  (CallFunction|ResetMaterials))

(event Custom|FreezeTime
  (params (SpecialDamageStruct :type Special%20Damage%20Struct%20Structure))
  (Variables|Default|SetSlowDownFactor 0.01)
  (Variables|Default|SetDamageSpeed 1.0)
  (Variables|Default|SetDamageType (.type SpecialDamageStruct))
  (CallFunction|SetTimeDilation)
  (CallFunction|SetMaterials)
  (Utilities|FlowControl|RetriggerableDelay (.duration SpecialDamageStruct))
  (Variables|Default|SetSlowDownFactor 1.0)
  (CallFunction|SetTimeDilation)
  (CallFunction|ResetMaterials))

(event EventBeginPlay
  (bind _returnvalue (Transformation|GetAttachParent))
  (Utilities|FlowControl|Sequence
    (:then_0
      (bind _asskeletal_mesh_component (Utilities|Casting|CastToSkeletalMeshComponent _returnvalue)
        (:then
          (CallFunction|CreateMaterialInstancies (Rendering|Material|GetMaterials _asskeletal_mesh_component) _asskeletal_mesh_component))
        (:CastFailed
          (bind _asstatic_mesh_component (Utilities|Casting|CastToStaticMeshComponent _returnvalue))
          (CallFunction|CreateMaterialInstancies (Rendering|Material|GetMaterials _asstatic_mesh_component) _asstatic_mesh_component))))
    (:then_1
      (bind _ascharacter (Utilities|Casting|CastToCharacter (Components|GetOwner))
        (:then
          (Variables|Default|SetCharacterMovementComponent (Variables|/Script/Engine.Character|GetCharacterMovement _ascharacter)))
        (:CastFailed
          (bind _asprimitive_component (Utilities|Casting|CastToPrimitiveComponent (Variables|/Script/Engine.Actor|GetRootComponent (Components|GetOwner))))
          (Variables|Default|SetPrimitiveComponent _asprimitive_component))))))

(event EventHitbyPlayer
  (params (HitDirection :type Vector :default "0, 0, 0") (HitLocation :type Vector :default "0, 0, 0") (HitBone :type Name :default "None") (Damage :type Float%20%28single-precision%29) (SpecialDamage :type Special%20Damage%20Struct%20Structure) (bIsEnvironment :type Boolean))
  (Variables|Default|SetbIsEnvironmentDamage bIsEnvironment)
  (CallFunction|ApplySpecialDamage SpecialDamage HitLocation))

(event EventPause
  (Variables|Default|SetPauseFactor 0.0)
  (CallFunction|SetTimeDilation)
  (Collision|SetActorEnableCollision (Components|GetOwner) false))

(event EventUnpause
  (Variables|Default|SetPauseFactor 1.0)
  (CallFunction|SetTimeDilation)
  (Collision|SetActorEnableCollision (Components|GetOwner) true))

(fn CreateMaterialInstancies
  (params (Materials :type Array%20of%20Material%20Interface%20Object%20References) (ActorComponent :type Primitive%20Component%20Object%20Reference))
  (for (_array_element _array_index) Materials
    (bind _returnvalue (Rendering|Material|CreateDynamicMaterialInstance ActorComponent _array_index _array_element "None" :!class /Script/Engine.PrimitiveComponent))
    (Utilities|Array|Add (Variables|Default|GetMI_Mesh) _returnvalue)))

(fn DamageTick
  (CallFunction|SetMaterials)
  (CallFunction|SetHealth))

(fn ResetMaterials
  (for _array_element (Variables|Default|GetMI_Mesh)
    (Rendering|Material|SetScalarParameterValue _array_element "PulseEmissiveAmount" 0.0 :!class /Script/Engine.MaterialInstanceDynamic)
    (Rendering|Material|SetVectorParameterValue :self _array_element :ParameterName "PulseColor" :!class /Script/Engine.MaterialInstanceDynamic)
    (Rendering|Material|SetScalarParameterValue _array_element "PulseSpeed" 1.0 :!class /Script/Engine.MaterialInstanceDynamic)))

(fn ForceTick
  (bind _returnvalue (Transformation|GetWorldLocation))
  (bind _charactermovementcomponent (Variables|Default|GetCharacterMovementComponent))
  (bind _hit_location (Variables|Default|GetHit%20Location))
  (bind _primitivecomponent (Variables|Default|GetPrimitiveComponent))
  (bind _returnvalue_2 (Math|Rotator|FindLookatRotation _returnvalue _hit_location))
  (bind _returnvalue_3 (Math|Vector|GetForwardVector _returnvalue_2))
  (bind _returnvalue_4 (* _returnvalue_3 4e+02))
  (CallFunction|SetMaterials)
  (Utilities|FlowControl|Sequence
    (:then_0
      (Utilities|IsValid _charactermovementcomponent
        (:Is%20Valid
          (Physics|AddImpulse _charactermovementcomponent _returnvalue_4 true))))
    (:then_1
      (Utilities|IsValid (Variables|Default|GetPrimitiveComponent)
        (:Is%20Valid
          (if (Physics|IsSimulatingPhysics _primitivecomponent "None")
            (Physics|AddImpulse _primitivecomponent _returnvalue_4 "None" true)))))))

(fn SetMaterials
  (for _array_element (Variables|Default|GetMI_Mesh)
    (Rendering|Material|SetScalarParameterValue _array_element "PulseEmissiveAmount" 1.0 :!class /Script/Engine.MaterialInstanceDynamic)
    (Rendering|Material|SetVectorParameterValue _array_element "PulseColor" (Utilities|Select :Index (Variables|Default|GetDamageType) :NewEnumerator8 "(R=1.000000,G=1.000000,B=1.000000,A=1.000000)" :NewEnumerator0 "(R=1.000000,G=0.074631,B=0.000000,A=1.000000)" :NewEnumerator1 "(R=0.000000,G=0.046303,B=0.421875,A=1.000000)" :NewEnumerator2 "(R=0.163719,G=1.000000,B=0.000000,A=1.000000)" :NewEnumerator3 "(R=1.000000,G=1.000000,B=0.000000,A=1.000000)" :NewEnumerator4 "(R=0.642485,G=0.000000,B=1.000000,A=1.000000)" :NewEnumerator5 "(R=0.078125,G=0.019145,B=0.000000,A=1.000000)" :NewEnumerator6 "(R=1.000000,G=0.871168,B=0.000000,A=1.000000)" :NewEnumerator7 "(R=1.000000,G=0.000000,B=0.000000,A=1.000000)") :!class /Script/Engine.MaterialInstanceDynamic)
    (Rendering|Material|SetScalarParameterValue _array_element "PulseSpeed" (Variables|Default|GetDamageSpeed) :!class /Script/Engine.MaterialInstanceDynamic)))

(fn SetBlackboardCanMove
  (params (bCanMove? :type Boolean))
  (bind _returnvalue (Components|GetOwner))
  (bind _returnvalue_2 (AI|GetBlackboard _returnvalue))
  (Utilities|IsValid _returnvalue_2
    (:Is%20Valid
      (AI|Components|Blackboard|SetValueasBool _returnvalue_2 (Utilities|Name|MakeLiteralName "bCanMove") bCanMove?))))

(fn SetTimeDilation
  (Variables|/Script/Engine.Actor|SetCustomTimeDilation (Components|GetOwner) (* (Variables|Default|GetPauseFactor) (Variables|Default|GetSlowDownFactor))))

(fn SetHealth
  (Class|BPIHitbyPlayer|ApplyDamageOverTime(Message) (Components|GetOwner) (Variables|Default|GetDamage)))