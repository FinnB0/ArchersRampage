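; Component that awards XP for its owning actor, adding it to the GS_SpellShot score and showing it as orange floating text.
; GetXP optionally adds a distance bonus to base XP, about 5 points per 5 meters from the player within a clamped range.
; CalculateXP then stacks critical, environment and stealth multipliers and rounds up, while JustXP bypasses both steps.
; A BP_DamageVisualizer spawned at an offset from the owner displays the result.
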(fn GetXP
  (bind _distancexp (CallFunction|CalculateDistanceAdditionXP))
  (bind _bjustxp (Variables|Default|GetbJustXP))
  (bind _xp (Variables|Default|GetXP))
  (bind _xp_2 (Variables|Default|GetXP))
  (bind _returnvalue (+ _distancexp _xp_2))
  (bind _calculatedxp (CallFunction|CalculateXP _returnvalue))
  (bind _returnvalue_2 (Math|Integer|SelectInt _xp _calculatedxp _bjustxp))
  (bind _asgs_spell_shot (Utilities|Casting|CastToGS_SpellShot (Game|GetGameState)))
  (Default|IncreaseScore _asgs_spell_shot _returnvalue_2)
  (Game|SpawnActorfromClass "/Game/Blueprints/BP_DamageVisualizer.BP_DamageVisualizer_C" (Math|Transform|MakeTransform (+ (Transformation|GetActorLocation (Components|GetOwner)) (Variables|Default|GetVizualizerOffset)) "0, 0, 0" "1,1,1") "AlwaysSpawn" 0 (Utilities|Text|ToText(String) (Utilities|String|Append (Utilities|String|ToString(Integer) _returnvalue_2) " XP")) (Utilities|Struct|MakeSlateColor "(R=1.000000,G=0.500000,B=0.000000,A=1.000000)") (Variables|Default|GetVizualizerScale) 0))

(fn CalculateDistanceAdditionXP
  ;[1 1 1] Get the Distance between the Player and the HitTarget for every 5 meter the player gets 5 extra XP
  (if (Variables|Default|GetbDistanceMultiplier)
    (return (* (Math|Float|Round (* (Math|Float|Clamp(Float) (Math|Vector|Distance(Vector) (Transformation|GetActorLocation (Components|GetOwner)) (Transformation|GetActorLocation (Game|Player|GetPlayerPawn 0))) (Variables|Default|GetMinDistance) (Variables|Default|GetMaxDistance)) 0.002)) 5))
    (else
      (return 0))))

(fn CalculateXP
  (params (XP :type Integer))
  (return (Math|Float|Ceil (* (* (* XP (Math|Float|SelectFloat (Variables|Default|GetCriticalMultiplier) 1.0 (Variables|Default|GetbIsCriticalDamage))) (Math|Float|SelectFloat (Variables|Default|GetEnvironmentMultiplier) 1.0 (Variables|Default|GetbIsEnvironmentDamage))) (Math|Float|SelectFloat (Variables|Default|GetStealthMultiplier) 1.0 (Variables|Default|GetbIsStealthDamage))))))