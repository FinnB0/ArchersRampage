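; Actor component that steers a flying AI Character toward a goal location by local trace-based avoidance, without a navmesh.
; On each interval-throttled tick it fires debug-drawn capsule traces in a horizontal ring with random pitch jitter.
; The unblocked endpoint nearest the goal becomes the next point.
; Until within minimum goal distance, it sets velocity toward that point at max fly speed and turns the AI controller to face it.
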(event EventBeginPlay
  (Class|ActorComponent|SetComponentTickInterval (Variables|Default|GetTickInterval)))

(event EventTick
  (params (DeltaSeconds :type Float%20%28single-precision%29))
  (bind _returnvalue (Components|GetOwner))
  (bind _ascharacter (Utilities|Casting|CastToCharacter _returnvalue))
  (bind _returnvalue_2 (Transformation|GetActorLocation _ascharacter))
  (bind _charactermovement (Variables|/Script/Engine.Character|GetCharacterMovement _ascharacter))
  (bind _ascharacter_2 (Utilities|Casting|CastToCharacter (Components|GetOwner)))
  (for _index (range 0 (Variables|Default|GetAmountOf%20Traces))
    (bind _outhit (Class|KismetSystemLibrary|CapsuleTraceSingleforObjects (Transformation|GetActorLocation _ascharacter_2) (+ (Transformation|GetActorLocation _ascharacter_2) (* (Math|Vector|GetForwardVector (Math|Rotator|MakeRotator 0.0 (Math|Random|RandomFloatinRange -2e+01 2e+01) (Math|Conversions|ToFloat(Integer) (* (/ 360 (Variables|Default|GetAmountOf%20Traces)) _index)))) (Variables|Default|GetTraceLenght))) (Variables|/Script/Engine.CapsuleComponent|GetCapsuleRadius (Variables|/Script/Engine.Character|GetCapsuleComponent _ascharacter_2)) (Variables|/Script/Engine.CapsuleComponent|GetCapsuleHalfHeight (Variables|/Script/Engine.Character|GetCapsuleComponent _ascharacter_2)) (Variables|Default|GetTracedObjectTypes) false 0 "ForDuration" true "(R=1.000000,G=0.000000,B=0.000000,A=1.000000)" "(R=0.000000,G=1.000000,B=0.000000,A=1.000000)" (Variables|Default|GetTickInterval)))
    (if (not (.bBlockingHit (Collision|BreakHitResult _outhit)))
      (if (< (Math|Vector|Distance(Vector) (.TraceEnd (Collision|BreakHitResult _outhit)) (Variables|Default|GetGoalLocation)) (Variables|Default|GetNearestLookAt))
        (Variables|Default|SetNearestLookAt (Math|Vector|Distance(Vector) (.TraceEnd (Collision|BreakHitResult _outhit)) (Variables|Default|GetGoalLocation)))
        (Variables|Default|SetNextLocationPoint (.TraceEnd (Collision|BreakHitResult _outhit))))))
  (Variables|Default|SetNearestLookAt 1e+06)
  (if (>= (Math|Vector|Distance(Vector) _returnvalue_2 (Variables|Default|GetGoalLocation)) (Variables|Default|GetMinGoalDistance))
    (Variables|/Script/Engine.MovementComponent|SetVelocity _charactermovement (* (Math|Vector|GetForwardVector (Math|Rotator|FindLookatRotation _returnvalue_2 (Variables|Default|GetNextLocationPoint))) (Variables|/Script/Engine.CharacterMovementComponent|GetMaxFlySpeed _charactermovement)))
    (Pawn|SetControlRotation (AI|GetAIController _ascharacter) (Math|Rotator|FindLookatRotation _returnvalue_2 (Variables|Default|GetNextLocationPoint)))))