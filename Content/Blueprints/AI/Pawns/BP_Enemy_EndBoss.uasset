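; Boss enemy pawn that plays an appearance montage on spawn before its behavior tree lets it move.
; On BeginPlay it calls GetGI, sets the AI controller's navigation filter and starts the behavior tree.
; The intro clears the bCanMove blackboard key, records StartLocation and turns the controller's yaw toward the player camera, then re-enables movement when the montage completes.
; An unconnected node would set bCanAttack.
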(event Custom|EndbossAppearing
  (bind _returnvalue (AI|GetBlackboard 0))
  (AI|Components|Blackboard|SetValueasBool _returnvalue (Utilities|Name|MakeLiteralName "bCanMove") false)
  (AI|Components|Blackboard|SetValueasVector _returnvalue (Utilities|Name|MakeLiteralName "StartLocation") (Transformation|GetActorLocation))
  (Pawn|SetControlRotation (Pawn|GetController) (Math|Rotator|MakeRotator 0.0 0.0 (.yaw (Math|Rotator|FindLookatRotation (Transformation|GetActorLocation) (Camera|GetCameraLocation (Game|GetPlayerCameraManager 0))))))
  (Animation|Montage|PlayMontage (Variables|Character|GetMesh) (Variables|Default|GetAppeareMontage)
    (:OnCompleted
      (AI|Components|Blackboard|SetValueasBool (AI|GetBlackboard 0) (Utilities|Name|MakeLiteralName "bCanMove") true))))

(event EventBeginPlay
  (bind _self self)
  (bind _returnvalue (AI|GetAIController _self))
  (CallFunction|GetGI)
  (Variables|/Script/AIModule.AIController|SetDefaultNavigationFilterClass _returnvalue (Variables|Default|GetQueryFilter))
  (AI|RunBehaviorTree _returnvalue (Variables|Default|GetBehaviorTree))
  (CallFunction|EndbossAppearing))

(fn ConstructionScript
  (|CallParentFunction))