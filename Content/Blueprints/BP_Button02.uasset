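; BP_Button02 is a shootable button that shows a configurable symbol and color.
; When a Projectile overlaps its skeletal mesh, it calls CallHitButton and plays a one-shot press animation.
; The construction script sets the text render's symbol and color and creates a dynamic material instance on the Bloom component to give its emissive color the same value.
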(event OnComponentBeginOverlap(SkeletalMesh)
  (params (OverlappedComponent :type Primitive%20Component%20Object%20Reference) (OtherActor :type Actor%20Object%20Reference) (OtherComp :type Primitive%20Component%20Object%20Reference) (OtherBodyIndex :type Integer) (bFromSweep :type Boolean) (SweepResult :type Hit%20Result%20Structure%20%28by%20ref%29))
  (Utilities|Casting|CastToProjectile OtherActor)
  (Default|CallHitButton)
  (Components|Animation|PlayAnimation (Variables|Default|GetSkeletalMesh) "/Game/Meshes/Buttons/Button02_Anim01.Button02_Anim01" false))

(fn ConstructionScript
  (bind _textrender (Variables|Default|GetTextRender))
  (bind _color (Variables|Default|GetColor))
  (bind _bloom (Variables|Default|GetBloom))
  (bind _returnvalue (Rendering|Material|CreateDynamicMaterialInstance _bloom 0 (Rendering|Material|GetMaterial _bloom 0) "None" :!class /Script/Engine.PrimitiveComponent))
  (Variables|Default|SetM_Bloom _returnvalue)
  (Rendering|Components|TextRender|SetText _textrender (Variables|Default|GetSymbol))
  (Rendering|Components|TextRender|SetTextRenderColor _textrender (Math|Conversions|ToColor(LinearColor) _color false))
  (Rendering|Material|SetVectorParameterValue (Variables|Default|GetM_Bloom) "EmissiveColor" _color :!class /Script/Engine.MaterialInstanceDynamic))