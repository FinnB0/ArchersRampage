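; Splash damage component that applies special damage to enemies and interactables within a radius of a hit location.
; SplashDamage sphere-traces WorldDynamic and PhysicsBody objects, gathers unique actors tagged Enemy or interact, then calls ApplySpecialDamage on each one's BP_SpecialDamageComponent.
; Regular Damage, IsEnvironment and IsOnlySpecialDamage have no effect, as the directional HitByPlayerMessage branch is disconnected.
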(fn SplashDamage
  (params (HitLocation :type Vector) (Radius :type Float%20%28single-precision%29) (Damage :type Float%20%28single-precision%29) (SpecialDamage :type Special%20Damage%20Struct%20Structure) (bIsEnvironment :type Boolean) (bIsOnlySpecialDamage :type Boolean))
  (bind _outhits (Collision|MultiSphereTraceForObjects HitLocation HitLocation Radius (Utilities|Array|MakeArray "ObjectTypeQuery2" "ObjectTypeQuery4") false 0 "None"))
  (for _array_element _outhits
    (if (or (Actor|ActorHasTag (.HitActor (Collision|BreakHitResult _array_element)) "Enemy") (Actor|ActorHasTag (.HitActor (Collision|BreakHitResult _array_element)) "interact"))
      (Utilities|Array|AddUnique (LocalVariables|GetDamagedActors) (.HitActor (Collision|BreakHitResult _array_element)))))
  (for _array_element_2 (LocalVariables|GetDamagedActors)
    (Utilities|IsValid (Actor|GetComponentbyClass _array_element_2 "/Game/Blueprints/AI/BP_SpecialDamageComponent.BP_SpecialDamageComponent_C")
      (:Is%20Valid
        (Default|ApplySpecialDamage (Actor|GetComponentbyClass _array_element_2 "/Game/Blueprints/AI/BP_SpecialDamageComponent.BP_SpecialDamageComponent_C") SpecialDamage HitLocation))))
  (Utilities|Array|Clear (LocalVariables|GetDamagedActors)))