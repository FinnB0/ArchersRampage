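; BP_PlayerState is a player state Blueprint that manages Steam achievements and stats for the game.
; It caches GI_SpellShot on BeginPlay, and each Steam event proceeds only if that instance is online and RequestCurrentStats succeeds.
; Events unlock an achievement, increment an integer stat or clear all listed achievements for testing.
; Another event zeroes one-turn stats whose index-matched achievement in a parallel array is still locked.
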(event Custom|SetSteamStat
  (params (StatName :type String) (AddValue :type Integer))
  ;[1 0.6 0] Get Achievement Function
  (if (Variables|/Game/Blueprints/GI_SpellShot.GI_SpellShot_C|GetbIsOnline (Variables|Default|GetGI))
    (bind _returnvalue (Class|UserStats|RequestCurrentStats))
    (if _returnvalue
      (bind (_data _returnvalue_2) (Class|UserStats|GetStatInt StatName))
      (if _returnvalue_2
        (Class|UserStats|SetStatInt StatName (+ _data AddValue))))))

(event Custom|SetSteamAchievement
  (params (AchievementName :type String))
  ;[1 0.6 0] Get Achievement Function
  (if (Variables|/Game/Blueprints/GI_SpellShot.GI_SpellShot_C|GetbIsOnline (Variables|Default|GetGI))
    (bind _returnvalue (Class|UserStats|RequestCurrentStats))
    (if _returnvalue
      (Class|UserStats|SetAchievement AchievementName))))

(event Custom|ResetAchievementsTEST
  ;[1 0.6 0] Get Achievement Function
  (if (Variables|/Game/Blueprints/GI_SpellShot.GI_SpellShot_C|GetbIsOnline (Variables|Default|GetGI))
    (bind _returnvalue (Class|UserStats|RequestCurrentStats))
    (if _returnvalue
      (for _array_element (Variables|Default|GetAchievements)
        (Class|UserStats|ClearAchievement _array_element)))))

(event Custom|ResetUnfinishedSteamStates
  ;[1 0.6 0] Get Achievement Function
  (if (Variables|/Game/Blueprints/GI_SpellShot.GI_SpellShot_C|GetbIsOnline (Variables|Default|GetGI))
    (bind _returnvalue (Class|UserStats|RequestCurrentStats))
    (if _returnvalue
      (for (_array_element _array_index) (Variables|Default|GetSteamOneTurnStates)
        (bind _bachieved (Class|UserStats|GetAchievement (Utilities|Array|Get(acopy) (Variables|Default|GetSteamOneTurnAchievements) _array_index)))
        (if (not _bachieved)
          (Class|UserStats|SetStatInt _array_element))))))

(event EventBeginPlay
  (CallFunction|GetGI))

(fn ConstructionScript)

(fn GetGI
  (bind _asgi_spell_shot (Utilities|Casting|CastToGI_SpellShot (Game|GetGameInstance)))
  (Variables|Default|SetGI _asgi_spell_shot))