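; GS_SpellShot appears to be the game state for SpellShot, tracking score and level completion time.
; IncreaseScore adds an increment to Score and clamps the result between zero and a fixed maximum.
; SetLevelStartTime records the current game time, and SetLevelEndTime subtracts it from the current time, so LevelEndTime stores and returns elapsed duration rather than a timestamp.
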(event Custom|IncreaseScore
  (params (Increasement :type Integer))
  (Variables|Default|SetScore (Math|Integer|Clamp(Integer) (+ (Variables|Default|GetScore) Increasement) 0 100000000)))

(fn ConstructionScript)

(fn SetLevelEndTime
  (bind _output_get (Variables|Default|SetLevelEndTime (- (Utilities|Time|GetGameTimeinSeconds) (Variables|Default|GetLevelStartTime))))
  (return _output_get))

(fn SetLevelStartTime
  (Variables|Default|SetLevelStartTime (Utilities|Time|GetGameTimeinSeconds)))