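; Exploding barrel actor that deals splash damage to nearby enemies when it receives damage of a matching type.
; A one-shot gate triggers SplashDamage, which sphere-traces for pawns within the damage radius and collects unique actors tagged Enemy.
; Each receives an ApplyDamage message with a hit direction pointing away from the barrel, then the barrel destroys itself.
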(event Custom|SplashDamage
  (bind _returnvalue (Transformation|GetActorLocation))
  (bind _returnvalue_2 (Transformation|GetActorLocation))
  (bind _outhits (Collision|MultiSphereTraceForObjects _returnvalue_2 _returnvalue_2 (Variables|Default|GetDamageRadius) (Utilities|Array|MakeArray "ObjectTypeQuery3") false 0 "None"))
  (for _array_element _outhits
    (if (Actor|ActorHasTag (.HitActor (Collision|BreakHitResult _array_element)) "Enemy")
      (Utilities|Array|AddUnique (Variables|Default|GetDamagedActors) (.HitActor (Collision|BreakHitResult _array_element)))))
  (for _array_element_2 (Variables|Default|GetDamagedActors)
    (Class|BPIDamage|ApplyDamage(Message) _array_element_2 (Math|Vector|GetForwardVector (Math|Rotator|FindLookatRotation _returnvalue (Transformation|GetActorLocation _array_element_2))) _returnvalue "None" (Variables|Default|GetDefaultDamage) (Variables|Default|GetDamageType) 1.0))
  (Utilities|Array|Clear (Variables|Default|GetDamagedActors))
  (Actor|DestroyActor))

(event EventApplyDamage
  (params (HitDirection :type Vector :default "0, 0, 0") (HitLocation :type Vector :default "0, 0, 0") (HitBone :type Name :default "None") (Damage :type Float%20%28single-precision%29) (DamageType :type DamageType%20Enum :default "NewEnumerator8") (EffectMultiplier :type Float%20%28single-precision%29))
  (if (Utilities|Enum|Equal(Enum) DamageType (Variables|Default|GetDamageType))
    (Utilities|FlowControl|DoOnce false
      (:Completed
        (CallFunction|SplashDamage)))))

(fn ConstructionScript)