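; Game instance for SpellShot that holds session-wide state: streamed levels and menus, pause state, difficulty options and scores.
; Init applies performance console commands, and difficulty toggles add or subtract their multipliers from the bonus XP.
; SaveScore re-sorts the local save-game leaderboard and uploads to Steam, whose top entries are fetched asynchronously to refresh scoreboards.
; A retriggerable delay resets the capped combo-kill counter, with a shorter window as it grows.
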(event Custom|AddCombiKill
  ;[1 1 1] Combi Kills
  (if (< (Variables|Default|GetCombiKillAmount) 5)
    (Math|Integer|IncrementInt (Variables|Default|GetCombiKillAmount)
      (:%20%20
        _)))
  (Default|CallAddCombiKills)
  (Utilities|FlowControl|RetriggerableDelay (/ 5.0 (Math|Conversions|ToFloat(Integer) (Variables|Default|GetCombiKillAmount))))
  (Variables|Default|SetCombiKillAmount 0)
  (Default|CallResetCombiKills))

(event Custom|LoadLevel
  (params (LevelName :type Name) (GameState :type GameState%20Enum :default "NewEnumerator0"))
  (Variables|Default|SetCurrentGameState GameState)
  (if (Utilities|Name|NotEqual(Name) (Variables|Default|GetCurrentLevel) "None")
    (Game|UnloadStreamLevel(byName) (Variables|Default|GetCurrentLevel) false))
  (Game|LoadStreamLevel(byName) LevelName true)
  (Variables|Default|SetCurrentLevel LevelName)
  (Class|BPICameraFade|Fadein(Message) (Game|Player|GetPlayerPawn 0))
  (bind _asgs_spell_shot (Utilities|Casting|CastToGS_SpellShot (Game|GetGameState)))
  (Default|SetLevelStartTime _asgs_spell_shot))

(event Custom|SaveScore
  (bind _localleaderboardtemp (Variables|Leaderboard|GetLocalLeaderboardTemp))
  (bind _asgs_spell_shot (Utilities|Casting|CastToGS_SpellShot (Game|GetGameState)))
  (Variables|Leaderboard|SetScore (+ (Variables|/Game/Blueprints/GS_SpellShot.GS_SpellShot_C|GetScore _asgs_spell_shot) (Variables|/Game/Blueprints/GS_SpellShot.GS_SpellShot_C|GetTimeScore _asgs_spell_shot)))
  (Utilities|FlowControl|Sequence
    (:then_0
      (Utilities|Array|Clear (Variables|Leaderboard|GetLocalLeaderboardTemp))
      (Variables|Leaderboard|SetLocalPlayerScore (Utilities|Struct|MakePlayerScore (Variables|Leaderboard|GetLocalPlayerName) (Math|DateTime|Now) (Variables|Leaderboard|GetScore) true))
      (bind _returnvalue (SaveGame|LoadGamefromSlot (Variables|Leaderboard|GetLeaderboard%20Name)))
      (bind _aslocal_score_save (Utilities|Casting|CastToLocalScoreSave _returnvalue)
        (:then
          (for (_array_element _array_index) (Variables|/Game/Blueprints/Scoresystem/LocalScoreSave.LocalScoreSave_C|GetLocalPlayerScores _aslocal_score_save)
            (if (Math|Boolean|ORBoolean (.isPlaying? (Utilities|Struct|BreakPlayerScore _array_element)) (== (.Score (Utilities|Struct|BreakPlayerScore _array_element)) 0) (>= _array_index 10))
              (Utilities|Array|RemoveItem (Variables|/Game/Blueprints/Scoresystem/LocalScoreSave.LocalScoreSave_C|GetLocalPlayerScores _aslocal_score_save) _array_element)))
          (Utilities|Array|Add (Variables|/Game/Blueprints/Scoresystem/LocalScoreSave.LocalScoreSave_C|GetLocalPlayerScores _aslocal_score_save) (Variables|Leaderboard|GetLocalPlayerScore))
          (for (_array_element_2 _array_index_2) (Variables|/Game/Blueprints/Scoresystem/LocalScoreSave.LocalScoreSave_C|GetLocalPlayerScores _aslocal_score_save)
            (for _index (range _array_index_2 (- (Utilities|Array|Length (Variables|/Game/Blueprints/Scoresystem/LocalScoreSave.LocalScoreSave_C|GetLocalPlayerScores _aslocal_score_save)) 1))
              (if (> (Utilities|Struct|BreakPlayerScore (Utilities|Array|Get(acopy) (Variables|/Game/Blueprints/Scoresystem/LocalScoreSave.LocalScoreSave_C|GetLocalPlayerScores _aslocal_score_save) _index)) (Utilities|Struct|BreakPlayerScore _array_element_2))
                (Utilities|Array|Swap (Variables|/Game/Blueprints/Scoresystem/LocalScoreSave.LocalScoreSave_C|GetLocalPlayerScores _aslocal_score_save) _index _array_index_2)))
            (Utilities|Array|Clear _localleaderboardtemp)
            (Utilities|Array|AppendArray _localleaderboardtemp (Variables|/Game/Blueprints/Scoresystem/LocalScoreSave.LocalScoreSave_C|GetLocalPlayerScores _aslocal_score_save))))
        (:CastFailed
          (Utilities|Array|Add (Variables|Leaderboard|GetLocalLeaderboardTemp) (Variables|Leaderboard|GetLocalPlayerScore))))
      (bind _returnvalue_2 (SaveGame|CreateSaveGameObject "/Game/Blueprints/Scoresystem/LocalScoreSave.LocalScoreSave_C"))
      (Utilities|Array|Clear (Variables|/Game/Blueprints/Scoresystem/LocalScoreSave.LocalScoreSave_C|GetLocalPlayerScores _returnvalue_2))
      (Utilities|Array|AppendArray (Variables|/Game/Blueprints/Scoresystem/LocalScoreSave.LocalScoreSave_C|GetLocalPlayerScores _returnvalue_2) (Variables|Leaderboard|GetLocalLeaderboardTemp))
      (SaveGame|SaveGametoSlot _returnvalue_2 (Variables|Leaderboard|GetLeaderboard%20Name)))
    (:then_1
      (|UploadLeaderboardScoreAsync (Variables|Leaderboard|GetSteamLeaderboard) "KeepBest" (Variables|Leaderboard|GetScore) 0 1e+01))))

(event Custom|GetSteamLeaderboard
  ;[1 1 1] Get Steam Leaderboards
  (Utilities|Array|Clear (Variables|Leaderboard|GetSteamEntries))
  (bind _data (|FindLeaderboardAsync (Variables|Leaderboard|GetLeaderboard%20Name) 1e+01)
    (:OnCallback
      (bind _data_2 (|DownloadLeaderboardEntriesAsync (.steamleaderboard _data) "Global" 0 20 1e+01)
        (:OnCallback
          (Variables|Leaderboard|SetSteamLeaderboard (.steamleaderboard _data_2))
          (for _index (range 0 19)
            (bind _leaderboardentry (Class|UserStats|GetDownloadedLeaderboardEntry (.steamleaderboardentries _data_2) _index))
            (Utilities|Array|Add (Variables|Leaderboard|GetSteamEntries) _leaderboardentry))
          (Default|CallRefreshScoreboards))))))

(event Custom|LoadMenu
  (params (MenuName :type Name) (bJustUnload :type Boolean))
  (if (Utilities|Name|NotEqual(Name) (Variables|Default|GetCurrentMenu) "None")
    (Game|UnloadStreamLevel(byName) (Variables|Default|GetCurrentMenu) false))
  (if bJustUnload
    (Variables|Default|SetCurrentMenu "None")
    (else
      (Game|LoadStreamLevel(byName) MenuName true)
      (Variables|Default|SetCurrentMenu MenuName))))

(event Custom|Unpause
  (Variables|Default|SetCurrentGameState (Variables|Default|GetLastGameState)))

(event Custom|Pause
  (Variables|Default|SetLastGameState (Variables|Default|GetCurrentGameState))
  (Variables|Default|SetCurrentGameState "NewEnumerator2"))

(event EventInit
  (CallFunction|SetPerformanceMedium))

(fn SetPerformanceMedium
  (for _array_element (Variables|Default|GetPerformanceCommands)
    (Development|ExecuteConsoleCommand _array_element 0)))

(fn SetGameSettingOption
  (params (bIsActive :type Boolean) (OptionIndex :type Integer))
  (switch int OptionIndex
    (:0
      (bind _output_get (Variables|Default|SetbBackQuiver bIsActive))
      (CallFunction|SetDifficultyBonusXP (Variables|Default|GetBackQuiverMultiplier) _output_get))
    (:1
      (bind _output_get_2 (Variables|Default|SetbOneLife bIsActive))
      (CallFunction|SetDifficultyBonusXP (Variables|Default|GetOneLifeMultiplier) _output_get_2)
      (Default|CallGameSettingOptionChangedOneLife _output_get_2))
    (:2
      (bind _output_get_3 (Variables|Default|SetbNoAimAssist bIsActive))
      (CallFunction|SetDifficultyBonusXP (Variables|Default|GetNoAimAssistMultiplier) _output_get_3))
    (:3
      (bind _output_get_4 (Variables|Default|SetbOnlyCrits bIsActive))
      (CallFunction|SetDifficultyBonusXP (Variables|Default|GetOnlyCritsMultiplier) _output_get_4))
    (:4
      (bind _output_get_5 (Variables|Default|SetbOneMinute bIsActive))
      (CallFunction|SetDifficultyBonusXP (Variables|Default|GetOneMinuteMultiplier) _output_get_5))
    (:5
      (bind _output_get_6 (Variables|Default|SetbMoreEnemies bIsActive))
      (CallFunction|SetDifficultyBonusXP (Variables|Default|GetMoreEnemiesMultiplier) _output_get_6))))

(fn SetDifficultyBonusXP
  (params (Multiplier :type Float%20%28single-precision%29) (bIsActive :type Boolean))
  (Variables|Default|SetDifficultyBonusXP (+ (Variables|Default|GetDifficultyBonusXP) (Math|Float|SelectFloat Multiplier (* Multiplier -1.0) bIsActive))))