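; BP_LevelPadLock is a padlock actor that sends the game to the level named in NewLevel when hit by the player.
; A one-shot HitbyPlayer event plays the unlock animation, enables physics, fades the pawn's message and changes GI_Achery's game state.
; After a delay it calls the game instance's LoadLevel, except "Questions", which sets QuestionTime and opens StartLevel.
; Pause and Unpause toggle the actor's collision.
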(event EventUnpause
  (Collision|SetActorEnableCollision true))

(event EventPause
  (Collision|SetActorEnableCollision false))

(event EventHitbyPlayer
  (params (HitDirection :type Vector :default "0, 0, 0") (HitLocation :type Vector :default "0, 0, 0") (HitBone :type Name :default "None") (Damage :type Float%20%28single-precision%29) (SpecialDamage :type Special%20Damage%20Struct%20Structure))
  (Utilities|FlowControl|DoOnce false
    (:Completed
      (Components|Animation|PlayAnimation (Variables|Default|GetSkeletalMesh) "/Game/Meshes/Padlock/Padlock_Anim.Padlock_Anim" false)
      (Physics|SetSimulatePhysics (Variables|Default|GetSkeletalMesh) true)
      (Class|BPICameraFade|FadeOut(Message) (Game|Player|GetPlayerPawn 0))
      (bind _asgi_achery (Utilities|Casting|CastToGI_Achery (Game|GetGameInstance)))
      (Variables|/Game/Blueprints/GI_Achery.GI_Achery_C|SetCurrentGameState _asgi_achery "NewEnumerator3")
      (Utilities|FlowControl|Delay 1.5)
      (bind _asgi_achery_2 (Utilities|Casting|CastToGI_Achery (Game|GetGameInstance)))
      (if (Utilities|Name|Equal(Name) (Variables|Default|GetNewLevel) "Questions")
        (Variables|/Game/Blueprints/GI_Achery.GI_Achery_C|SetQuestionTime? _asgi_achery_2 true)
        (Utilities|FlowControl|Delay 1.0)
        (Game|OpenLevel(byName) "StartLevel")
        (else
          (Default|LoadLevel _asgi_achery_2 (Variables|Default|GetNewLevel) "NewEnumerator0"))))))

(fn ConstructionScript)