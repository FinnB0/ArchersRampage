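; Teleport destination platform that pulls the player to itself when a BP_Projectile overlaps its cube.
; The TeleportTimer timeline is built to lerp the player from their captured location to the platform's origin, without sweeping.
; The same timeline drives saturation, contrast and global tint in MPC_ColorCorrection for a screen effect during the move.
; A platform flagged IsStartPlatform attaches the player pawn to itself on BeginPlay.
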(event OnComponentBeginOverlap(Cube)
  (params (OverlappedComponent :type Primitive%20Component%20Object%20Reference) (OtherActor :type Actor%20Object%20Reference) (OtherComp :type Primitive%20Component%20Object%20Reference) (OtherBodyIndex :type Integer) (bFromSweep :type Boolean) (SweepResult :type Hit%20Result%20Structure%20%28by%20ref%29))
  (Utilities|Casting|CastToBP_Projectile OtherActor)
  (Variables|Default|SetStartLocation (Transformation|GetActorLocation (Game|Player|GetPlayerPawn 0)))
  (Components|Timeline|PlayfromStart (Variables|Default|GetTeleportTimer)))

(event EventBeginPlay
  (if (Variables|Default|GetisStartPlatform?)
    (Transformation|AttachActorToActor (Game|Player|GetPlayerPawn 0) self "None" "KeepWorld" "KeepWorld" "KeepWorld" true)))

(fn ConstructionScript)