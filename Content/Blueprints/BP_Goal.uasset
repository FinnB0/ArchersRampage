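; BP_Goal is the end-of-level goal for a VR game, showing the score and providing the link to the next level.
; On BeginPlay it spawns a BP_Door at the entry socket, passing on its damage type and lock state.
; The first VRPawn overlap of GoalTrigger reveals and refreshes the HUD_Score widget, plays a success sound and spawns a BP_LevelPadLock carrying NextLevel.
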(event OnComponentBeginOverlap(GoalTrigger)
  (params (OverlappedComponent :type Primitive%20Component%20Object%20Reference) (OtherActor :type Actor%20Object%20Reference) (OtherComp :type Primitive%20Component%20Object%20Reference) (OtherBodyIndex :type Integer) (bFromSweep :type Boolean) (SweepResult :type Hit%20Result%20Structure%20%28by%20ref%29))
  (bind _widget (Variables|Default|GetWidget))
  (Utilities|Casting|CastToVRPawn OtherActor)
  (Utilities|FlowControl|DoOnce false
    (:Completed
      (Development|SetHiddeninGame _widget false false)
      (bind _ashud_score (Utilities|Casting|CastToHUD_Score (UserInterface|GetWidget _widget)))
      (Default|UpdateDisplay _ashud_score)
      (UserInterface|RequestRenderUpdate (Variables|Default|GetWidget))
      (Audio|PlaySound2D "/Game/Sounds/Success_Cue.Success_Cue" 1.0 1.0 0.0 0 (Game|Player|GetPlayerPawn 0))
      (Game|SpawnActorfromClass "/Game/Blueprints/BP_LevelPadLock.BP_LevelPadLock_C" (Transformation|GetWorldTransform (Variables|Default|GetNextLevelLockSocket)) "AlwaysSpawn" self (Variables|Default|GetNextLevel) 0))))

(event EventBeginPlay
  (Game|SpawnActorfromClass "/Game/Blueprints/BP_Door.BP_Door_C" (Transformation|GetWorldTransform (Variables|Default|GetEntryDoorSocket)) "Undefined" self (Variables|Default|GetDoorDamageType) (Variables|Default|GetIs%20Locked?) 0))

(fn ConstructionScript)