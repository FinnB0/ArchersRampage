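; Floating rock actor that reacts to one special damage type from player hits by flying toward the hit location.
; That hit starts a looping timer that applies repeated velocity-change impulses to its sphere, paused after a retriggerable delay.
; The construction script randomizes uniform scale and a dynamic material's rotation parameters and base color tint, so each rock varies.
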(event Custom|ForceTick
  (Physics|AddImpulse (Variables|Default|GetSphere) (* (Math|Vector|GetForwardVector (Math|Rotator|FindLookatRotation (Transformation|GetActorLocation) (Variables|Default|GetForce%20Direction))) 4e+02) "None" true))

(event EventHitbyPlayer
  (params (HitDirection :type Vector :default "0, 0, 0") (HitLocation :type Vector :default "0, 0, 0") (HitBone :type Name :default "None") (Damage :type Float%20%28single-precision%29) (SpecialDamage :type Special%20Damage%20Struct%20Structure))
  (if (Utilities|Enum|Equal(Enum) (.Type (Utilities|Struct|BreakSpecialDamageStruct SpecialDamage)) "NewEnumerator4")
    (Variables|Default|SetForce%20Direction HitLocation)
    (bind _returnvalue (Utilities|Time|SetTimerbyEvent (EventDispatchers|CreateEvent :!event Custom|ForceTick) 0.1 true))
    (Variables|Default|SetForceTimer _returnvalue)
    (Utilities|FlowControl|RetriggerableDelay 3.0)
    (Utilities|Time|PauseTimerbyHandle (Variables|Default|GetForceTimer))))

(fn ConstructionScript
  (CallFunction|CreateMaterialInstance)
  (CallFunction|SetMaterialParameters)
  (CallFunction|SetRandomScale))

(fn CreateMaterialInstance
  (bind _staticmesh (Variables|Default|GetStaticMesh))
  (bind _returnvalue (Rendering|Material|CreateDynamicMaterialInstance _staticmesh 0 (Rendering|Material|GetMaterial _staticmesh 0) "None" :!class /Script/Engine.PrimitiveComponent))
  (Variables|Default|SetMI_Rock _returnvalue))

(fn SetMaterialParameters
  (bind _mi_rock (Variables|Default|GetMI_Rock))
  (Rendering|Material|SetScalarParameterValue _mi_rock "RotationSpeed" (Math|Random|RandomFloatinRange -0.1 0.1) :!class /Script/Engine.MaterialInstanceDynamic)
  (Rendering|Material|SetVectorParameterValue _mi_rock "RotationVector" (Math|Conversions|ToLinearColor(Vector) (* (Math|Random|RandomUnitVector) (Math|Random|RandomFloatinRange -1.0 1.0))) :!class /Script/Engine.MaterialInstanceDynamic)
  (Rendering|Material|SetVectorParameterValue _mi_rock "BaseColorTint" (Utilities|Select :Index (Math|Random|RandomIntegerinRange 0 2) :Option%200 "(R=0.114583,G=0.069279,B=0.043566,A=1.000000)" :Option%201 "(R=0.093750,G=0.042974,B=0.009369,A=1.000000)" :Option%202 "(R=0.243137,G=0.133333,B=0.094118,A=1.000000)" :Option%203 "(R=0.151042,G=0.047065,B=0.031996,A=1.000000)") :!class /Script/Engine.MaterialInstanceDynamic))

(fn SetRandomScale
  (Transformation|SetActorScale3D (Math|Conversions|ToVector(Float) (Math|Random|RandomFloatinRange 1.0 1.2))))