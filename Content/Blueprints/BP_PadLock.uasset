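; Padlock that the player opens by hitting it with a matching special damage type, while a lock set to Normal accepts any hit.
; The first valid hit fires LockOpened, plays the unlock animation and enables physics simulation on the skeletal mesh.
; The construction script creates a dynamic material instance and sets the symbol texture, pulse and tint colors from DamageType.
; Pause and Unpause events toggle the actor's collision.
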(event EventUnpause
  (Collision|SetActorEnableCollision true))

(event EventPause
  (Collision|SetActorEnableCollision false))

(event EventHitbyPlayer
  (params (HitDirection :type Vector :default "0, 0, 0") (HitLocation :type Vector :default "0, 0, 0") (HitBone :type Name :default "None") (Damage :type Float%20%28single-precision%29) (SpecialDamage :type Special%20Damage%20Struct%20Structure))
  (if (or (Utilities|Enum|Equal(Enum) (.type SpecialDamage) (Variables|Default|GetDamageType)) (Utilities|Enum|Equal(Enum) (Variables|Default|GetDamageType) "NewEnumerator8"))
    (Utilities|FlowControl|DoOnce false
      (:Completed
        (Default|CallLockOpened)
        (Components|Animation|PlayAnimation (Variables|Default|GetSkeletalMesh) "/Game/Meshes/Padlock/Animations/Padlock_Anim.Padlock_Anim" false)
        (Physics|SetSimulatePhysics (Variables|Default|GetSkeletalMesh) true)))))

(fn ConstructionScript
  (bind _mi_padlock (Variables|Default|GetMI_PadLock))
  (bind _damagetype (Variables|Default|GetDamageType))
  (bind _returnvalue (Utilities|Select :Index _damagetype :NewEnumerator8 "(R=1.000000,G=1.000000,B=1.000000,A=1.000000)" :NewEnumerator0 "(R=1.000000,G=0.000000,B=0.000000,A=1.000000)" :NewEnumerator1 "(R=0.000000,G=0.329412,B=1.000000,A=1.000000)" :NewEnumerator2 "(R=0.533333,G=1.000000,B=0.000000,A=1.000000)" :NewEnumerator3 "(R=1.000000,G=1.000000,B=0.100000,A=1.000000)" :NewEnumerator4 "(R=0.725490,G=0.000000,B=1.000000,A=1.000000)" :NewEnumerator5 "(R=1.000000,G=0.505882,B=0.000000,A=1.000000)" :NewEnumerator6 "(R=0.000000,G=0.960784,B=1.000000,A=1.000000)" :NewEnumerator7 "(R=1.000000,G=0.000000,B=0.792157,A=1.000000)"))
  (CallFunction|CreateMaterialInstance)
  (Rendering|Material|SetTextureParameterValue _mi_padlock "Symbol" (Utilities|Select :Index _damagetype :NewEnumerator8 "/Game/Textures/HUD/T_Target_A.T_Target_A" :NewEnumerator0 "/Game/Textures/MagicSymbols/T_SymbolFire_A.T_SymbolFire_A" :NewEnumerator1 "/Game/Textures/MagicSymbols/T_SymbolIce_A.T_SymbolIce_A" :NewEnumerator2 "/Game/Textures/MagicSymbols/T_SymbolPoison_A.T_SymbolPoison_A" :NewEnumerator3 "/Game/Textures/MagicSymbols/T_SymbolElectricity_A.T_SymbolElectricity_A" :NewEnumerator4 "/Game/Textures/MagicSymbols/T_SymbolGravity_A.T_SymbolGravity_A" :NewEnumerator5 "/Game/Textures/MagicSymbols/T_SymbolExplosion_A.T_SymbolExplosion_A" :NewEnumerator6 "/Game/Textures/MagicSymbols/T_SymbolLuck_A.T_SymbolLuck_A" :NewEnumerator7 "/Game/Textures/MagicSymbols/T_SymbolSuck_A.T_SymbolSuck_A"))
  (Rendering|Material|SetVectorParameterValue _mi_padlock "SymbolColor" (Utilities|Select :Index _damagetype :NewEnumerator8 "(R=1.000000,G=1.000000,B=1.000000,A=1.000000)" :NewEnumerator0 "(R=1.000000,G=0.000000,B=0.000000,A=1.000000)" :NewEnumerator1 "(R=0.000000,G=0.329412,B=1.000000,A=1.000000)" :NewEnumerator2 "(R=0.533333,G=1.000000,B=0.000000,A=1.000000)" :NewEnumerator3 "(R=1.000000,G=1.000000,B=0.100000,A=1.000000)" :NewEnumerator4 "(R=0.725490,G=0.000000,B=1.000000,A=1.000000)" :NewEnumerator5 "(R=1.000000,G=0.505882,B=0.000000,A=1.000000)" :NewEnumerator6 "(R=0.000000,G=0.960784,B=1.000000,A=1.000000)" :NewEnumerator7 "(R=1.000000,G=0.000000,B=0.792157,A=1.000000)") :!class /Script/Engine.MaterialInstanceDynamic)
  (Rendering|Material|SetVectorParameterValue _mi_padlock "PulseColor" _returnvalue :!class /Script/Engine.MaterialInstanceDynamic)
  (Rendering|Material|SetVectorParameterValue _mi_padlock "BaseColorTint" (* _returnvalue 0.1) :!class /Script/Engine.MaterialInstanceDynamic))

(fn CreateMaterialInstance
  (bind _skeletalmesh (Variables|Default|GetSkeletalMesh))
  (bind _returnvalue (Rendering|Material|CreateDynamicMaterialInstance _skeletalmesh 0 (Rendering|Material|GetMaterial _skeletalmesh 0) "None" :!class /Script/Engine.PrimitiveComponent))
  (Variables|Default|SetMI_PadLock _returnvalue))