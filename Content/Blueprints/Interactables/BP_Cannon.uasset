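; BP_Cannon is an interactable cannon that fires when hit by a specific special damage type, up to InteractCount times.
; A hit awards XP and starts a timeline that animates the fuse through a dynamic material parameter, then spawns a projectile at ShotSocket.
; A DoOnce blocks retriggering until a delayed reset timeline restores the fuse, which is skipped after the final shot.
; Pause and Unpause toggle actor collision.
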(event Custom|FinishReset
  (Utilities|FlowControl|DoOnce false) ; enters at Reset
)

(event Custom|SpawnProjectile
  (params (AttackSocket :type Name))
  (bind _skeletalmesh (Variables|Default|GetSkeletalMesh))
  (bind _returnvalue (Transformation|GetSocketLocation _skeletalmesh AttackSocket))
  (Game|SpawnActorfromClass "/Game/Blueprints/Interactables/BP_Projectile_Cannon.BP_Projectile_Cannon_C" (Math|Transform|MakeTransform _returnvalue (Transformation|GetSocketRotation _skeletalmesh AttackSocket) "1,1,1") "Undefined" 0 (Variables|Default|GetDamage%20Projectile) self)
  (Audio|PlaySoundatLocation "/Game/Sounds/Enemy/EnemyShot01_Cue.EnemyShot01_Cue" _returnvalue "0, 0, 0" 1.0 1.0 0.0 0 0 0))

(event Custom|ResetCannon
  (if (!= (Variables|Default|GetCurrentInteractCounter) (Variables|Default|GetInteractCount))
    (Utilities|FlowControl|Delay 2.0)
    (bind _fusetrack (Timeline|ResetTimer PlayFromStart)
      (:Update
        (Rendering|Material|SetScalarParameterValue (Variables|Default|GetMI_Fuse) "CurrentCount" _fusetrack :!class /Script/Engine.MaterialInstanceDynamic))
      (:Finished
        (CallFunction|FinishReset)))))

(event Custom|StartShot
  (Default|GetXP (Variables|Default|GetBP_ExperienceCalculationComponent))
  (Components|Animation|PlayAnimation (Variables|Default|GetSkeletalMesh) "/Game/Meshes/Cannon/Cannon_BurnFuse.Cannon_BurnFuse" false)
  (bind _fusetrack (Timeline|ShotTimer PlayFromStart)
    (:Update
      (Rendering|Material|SetScalarParameterValue (Variables|Default|GetMI_Fuse) "CurrentCount" _fusetrack :!class /Script/Engine.MaterialInstanceDynamic))
    (:Finished
      (Components|Animation|PlayAnimation (Variables|Default|GetSkeletalMesh) "/Game/Meshes/Cannon/Cannon_Shot.Cannon_Shot" false)
      (CallFunction|SpawnProjectile "ShotSocket")
      (CallFunction|ResetCannon))))

(event EventUnpause
  (Collision|SetActorEnableCollision true))

(event EventPause
  (Collision|SetActorEnableCollision false))

(event EventBeginPlay
  (CallFunction|CreateMaterialInstance))

(event EventHit
  (params (HitDirection :type Vector :default "0, 0, 0") (HitLocation :type Vector :default "0, 0, 0") (HitBone :type Name :default "None") (DirectDamage :type Float%20%28single-precision%29) (SpecialDamage :type Special%20Damage%20Struct%20Structure) (DamageCauser :type DamageCauserType%20Enum :default "NewEnumerator0"))
  (if (Utilities|Enum|Equal(Enum) (Utilities|Struct|BreakSpecialDamageStruct SpecialDamage) "NewEnumerator0")
    (Utilities|FlowControl|DoOnce false
      (:Completed
        (bind _counter (Utilities|FlowControl|DoN (Variables|Default|GetInteractCount))
          (:Exit
            (Variables|Default|SetCurrentInteractCounter _counter)
            (CallFunction|StartShot)))))))

(fn ConstructionScript)

(fn CreateMaterialInstance
  (bind _skeletalmesh (Variables|Default|GetSkeletalMesh))
  (bind _returnvalue (Rendering|Material|CreateDynamicMaterialInstance _skeletalmesh 0 (Rendering|Material|GetMaterial _skeletalmesh 0) "None" :!class /Script/Engine.PrimitiveComponent))
  (Variables|Default|SetMI_Fuse _returnvalue))