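; BP_Container01 is an interactable container that opens when hit by the player and triggers connected enemy spawners.
; The first hit passes a DoOnce, plays the skeletal mesh animation without looping, then calls SpawnEnemy on every entry in ConnectedEnemySpawners.
; Pause and Unpause events toggle the actor's collision off and on.
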(event Custom|SpawnEnemys
  (bind _connectedenemyspawners (Variables|Default|GetConnectedEnemySpawners))
  (if (Utilities|Array|IsValidIndex _connectedenemyspawners)
    (for _array_element _connectedenemyspawners
      (Default|SpawnEnemy _array_element))))

(event EventUnpause
  (Collision|SetActorEnableCollision true))

(event EventPause
  (Collision|SetActorEnableCollision false))

(event EventHitbyPlayer
  (params (HitDirection :type Vector :default "0, 0, 0") (HitLocation :type Vector :default "0, 0, 0") (HitBone :type Name :default "None") (DirectDamage :type Float%20%28single-precision%29) (SpecialDamage :type Special%20Damage%20Struct%20Structure))
  (Utilities|FlowControl|DoOnce false
    (:Completed
      (Audio|Components|Audio|Play (Variables|Default|GetSkeletalMesh) false)
      (CallFunction|SpawnEnemys))))

(fn ConstructionScript)