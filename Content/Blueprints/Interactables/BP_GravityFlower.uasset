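; BP_GravityFlower is an interactable environmental hazard that sets off an area effect the first time the player hits it.
; The hit swaps the intact flower for its destroyed version, then triggers timed special splash damage from the Arrow's location through BPSplashDamageComponent, flagged as environmental.
; It also calls GetXP on BPExperienceCalculationComponent.
; Pause and Unpause events switch the actor's collision off and on.
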(event EventUnpause
  (Collision|SetActorEnableCollision true))

(event EventPause
  (Collision|SetActorEnableCollision false))

(event EventHitbyPlayer
  (params (HitDirection :type Vector :default "0, 0, 0") (HitLocation :type Vector :default "0, 0, 0") (HitBone :type Name :default "None") (DirectDamage :type Float%20%28single-precision%29) (SpecialDamage :type Special%20Damage%20Struct%20Structure))
  (Utilities|FlowControl|DoOnce false
    (:Completed
      (Development|SetHiddeninGame (Variables|Default|GetGravityFlower_Destroyed) false false)
      (Development|SetHiddeninGame (Variables|Default|GetGravityFlower) true false)
      (Default|SplashDamage (Variables|Default|GetBP_SplashDamageComponent) (Transformation|GetWorldLocation (Variables|Default|GetArrow)) 6e+02 0.0 (Utilities|Struct|MakeSpecialDamageStruct "NewEnumerator4" 1e+01 0.0 0.1) true)
      (Default|GetXP (Variables|Default|GetBP_ExperienceCalculationComponent)))))

(event EventBeginPlay)

(fn ConstructionScript)