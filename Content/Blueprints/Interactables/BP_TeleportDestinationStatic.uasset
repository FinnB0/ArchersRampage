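; A static VR teleport destination that moves the player pawn to its location when hit, then triggers every connected enemy spawner.
; Activate and Deactivate toggle collision, the border glow and an EmissiveAmount parameter on dynamic border materials.
; The construction script creates those material instances and applies the initial IsActivated state.
; Pause disables collision, and Unpause restores it only if IsActivated is set.
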(event Custom|SpawnEnemys
  (bind _connectedenemyspawners (Variables|Default|GetConnectedEnemySpawners))
  (if (Utilities|Array|IsValidIndex _connectedenemyspawners)
    (for _array_element _connectedenemyspawners
      (Default|SpawnEnemy _array_element))))

(event Custom|Activate
  (Development|SetHiddeninGame (Variables|Default|GetBorderGlow) false false)
  (Collision|SetActorEnableCollision true)
  (for _array_element (Variables|Default|GetMI_Border)
    (Rendering|Material|SetScalarParameterValue _array_element "EmissiveAmount" 1.0 :!class /Script/Engine.MaterialInstanceDynamic)))

(event Custom|Deactivate
  (Development|SetHiddeninGame (Variables|Default|GetBorderGlow) true false)
  (Collision|SetActorEnableCollision false)
  (for _array_element (Variables|Default|GetMI_Border)
    (Rendering|Material|SetScalarParameterValue _array_element "EmissiveAmount" 0.0 :!class /Script/Engine.MaterialInstanceDynamic)))

(event EventHitbyPlayer
  (params (HitDirection :type Vector :default "0, 0, 0") (HitLocation :type Vector :default "0, 0, 0") (HitBone :type Name :default "None") (DirectDamage :type Float%20%28single-precision%29) (SpecialDamage :type Special%20Damage%20Struct%20Structure))
  (Default|Teleport (.AsVRPawn (Utilities|Casting|CastToVRPawn (Game|Player|GetPlayerPawn 0))) (Transformation|GetActorLocation))
  (CallFunction|SpawnEnemys))

(event EventPause
  (Collision|SetActorEnableCollision false))

(event EventUnpause
  (if (Variables|Default|GetbIsActivated)
    (Collision|SetActorEnableCollision true)))

(fn ConstructionScript
  (CallFunction|CreateMaterialInstancies)
  (if (Variables|Default|GetbIsActivated)
    (CallFunction|Activate)
    (else
      (CallFunction|Deactivate))))

(fn CreateMaterialInstancies
  (for (_array_element _array_index) (Rendering|Material|GetMaterials (Variables|Default|GetBorder))
    (bind _returnvalue (Rendering|Material|CreateDynamicMaterialInstance (Variables|Default|GetBorder) _array_index _array_element "None" :!class /Script/Engine.PrimitiveComponent))
    (Utilities|Array|Add (Variables|Default|GetMI_Border) _returnvalue)))