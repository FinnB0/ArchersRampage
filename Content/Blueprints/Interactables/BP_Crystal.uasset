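; BP_Crystal is a breakable crystal interactable that rewards the player when hit.
; The first hit swaps the intact mesh for the destroyed one, disables the crystal's collision, plays a break sound and spawns a Niagara effect at SystemSpawnPoint.
; It then grants XP through BPExperienceCalculationComponent and increments a Steam stat on BP_PlayerState for achievements.
; Pause and Unpause events toggle the actor's collision off and on.
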(event EventUnpause
  (Collision|SetActorEnableCollision true))

(event EventPause
  (Collision|SetActorEnableCollision false))

(event EventHitbyPlayer
  (params (HitDirection :type Vector :default "0, 0, 0") (HitLocation :type Vector :default "0, 0, 0") (HitBone :type Name :default "None") (DirectDamage :type Float%20%28single-precision%29) (SpecialDamage :type Special%20Damage%20Struct%20Structure) (DamageCauser :type DamageCauserType%20Enum :default "NewEnumerator0"))
  (bind _systemspawnpoint (Variables|Default|GetSystemSpawnPoint))
  (bind _returnvalue (Transformation|GetWorldTransform _systemspawnpoint))
  (Utilities|FlowControl|DoOnce false
    (:Completed
      (Development|SetHiddeninGame (Variables|Default|GetCrystal_Destroyed) false false)
      (Development|SetHiddeninGame (Variables|Default|GetCrystal) true false)
      (Collision|SetCollisionEnabled (Variables|Default|GetCrystal) "NoCollision")
      (Audio|PlaySoundatLocation "/Game/Sounds/BreakCrystal_Cue.BreakCrystal_Cue" (.location _returnvalue) "0, 0, 0" 1.0 1.0 0.0 0 0 0)
      (Niagara|SpawnSystematLocation "/Game/Particles/NS_Crystal.NS_Crystal" (.location _returnvalue) (.rotation _returnvalue))
      (Default|GetXP (Variables|Default|GetBP_ExperienceCalculationComponent))
      (Achievements|AchievementBreakCrystal))))

(fn ConstructionScript)

(fn AchievementBreakCrystal
  (Default|SetSteamStat (.AsBP%20Player%20State (Utilities|Casting|CastToBP_PlayerState (Variables|/Script/Engine.Controller|GetPlayerState (Game|GetPlayerController 0)))) "crystal_crystal" 1))