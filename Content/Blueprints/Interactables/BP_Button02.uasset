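; BP_Button02 is a 3D menu-style button that reacts to player hits with a sound and, unless disabled, a press animation.
; An enabled hit fires the HitButton dispatcher, plus HitButtonInt when IntValue is not -1.
; The construction script creates dynamic materials for mesh and bloom and sets the label.
; Enable, disable and toggle events recolor materials and text for active, inactive or disabled states.
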(event Custom|EnableButton
  (bind _textcoloractive (Variables|Default|GetTextColorActive))
  (bind _textcolordeactive (Variables|Default|GetTextColorDeactive))
  (Variables|Default|SetbIsDisabled false)
  (if (Variables|Default|GetbIsActive)
    (Rendering|Material|SetVectorParameterValue (Variables|Default|GetM_Button) "DisplayColor" (Variables|Default|GetDisplayColorActive) :!class /Script/Engine.MaterialInstanceDynamic)
    (Rendering|Components|TextRender|SetTextRenderColor (Variables|Default|GetTextRender) (Math|Conversions|ToColor(LinearColor) _textcoloractive false))
    (Rendering|Material|SetVectorParameterValue (Variables|Default|GetM_Bloom) "EmissiveColor" _textcoloractive :!class /Script/Engine.MaterialInstanceDynamic)
    (else
      (Rendering|Material|SetVectorParameterValue (Variables|Default|GetM_Button) "DisplayColor" (Variables|Default|GetDisplayColorDeactive) :!class /Script/Engine.MaterialInstanceDynamic)
      (Rendering|Components|TextRender|SetTextRenderColor (Variables|Default|GetTextRender) (Math|Conversions|ToColor(LinearColor) _textcolordeactive false))
      (Rendering|Material|SetVectorParameterValue (Variables|Default|GetM_Bloom) "EmissiveColor" _textcolordeactive :!class /Script/Engine.MaterialInstanceDynamic))))

(event Custom|DisableButton
  (bind _disabledcolor (Variables|Default|GetDisabledColor))
  (Variables|Default|SetbIsDisabled true)
  (Rendering|Material|SetVectorParameterValue (Variables|Default|GetM_Button) "DisplayColor" _disabledcolor :!class /Script/Engine.MaterialInstanceDynamic)
  (Rendering|Components|TextRender|SetTextRenderColor (Variables|Default|GetTextRender) (Math|Conversions|ToColor(LinearColor) _disabledcolor false))
  (Rendering|Material|SetVectorParameterValue (Variables|Default|GetM_Bloom) "EmissiveColor" _disabledcolor :!class /Script/Engine.MaterialInstanceDynamic))

(event Custom|SwitchButtonActivity
  (if (Variables|Default|GetbIsActive)
    (Variables|Default|SetbIsActive false)
    (else
      (Variables|Default|SetbIsActive true)))
  (CallFunction|EnableButton))

(event EventHitbyPlayer
  (params (HitDirection :type Vector :default "0, 0, 0") (HitLocation :type Vector :default "0, 0, 0") (HitBone :type Name :default "None") (DirectDamage :type Float%20%28single-precision%29) (SpecialDamage :type Special%20Damage%20Struct%20Structure) (DamageCauser :type DamageCauserType%20Enum :default "NewEnumerator0"))
  (Audio|PlaySoundatLocation "/Game/Sounds/MenuHit_Cue.MenuHit_Cue" HitLocation "0, 0, 0" 1.0 1.0 0.0 0 0 0)
  (if (not (Variables|Default|GetbIsDisabled))
    (Default|CallHitButton)
    (Components|Animation|PlayAnimation (Variables|Default|GetSkeletalMesh) "/Game/Meshes/Buttons/Animations/Button02_Anim01.Button02_Anim01" false)
    (if (!= (Variables|Default|GetInt%20Value) -1)
      (Default|CallHitButtonInt (Variables|Default|GetInt%20Value) self))))

(fn ConstructionScript
  (CallFunction|CreateMaterialsInstancies)
  (Rendering|Components|TextRender|SetWorldSize (Variables|Default|GetTextRender) (Variables|Default|GetTextSize))
  (Rendering|Components|TextRender|SetText (Variables|Default|GetTextRender) (Variables|Default|GetSymbol))
  (if (Variables|Default|GetbIsDisabled)
    (CallFunction|DisableButton)
    (else
      (CallFunction|EnableButton))))

(fn CreateMaterialsInstancies
  (bind _skeletalmesh (Variables|Default|GetSkeletalMesh))
  (bind _bloom (Variables|Default|GetBloom))
  (bind _returnvalue (Rendering|Material|CreateDynamicMaterialInstance _skeletalmesh 0 (Rendering|Material|GetMaterial _skeletalmesh 0) "None" :!class /Script/Engine.PrimitiveComponent))
  (Variables|Default|SetM_Button _returnvalue)
  (bind _returnvalue_2 (Rendering|Material|CreateDynamicMaterialInstance _bloom 0 (Rendering|Material|GetMaterial _bloom 0) "None" :!class /Script/Engine.PrimitiveComponent))
  (Variables|Default|SetM_Bloom _returnvalue_2))