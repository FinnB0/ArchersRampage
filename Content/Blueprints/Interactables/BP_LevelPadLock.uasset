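; BP_LevelPadLock is a level-exit padlock in a VR game that ends the level when the player hits it.
; The first hit plays its animation, enables physics, fades out the player's message, saves the score and awards a Steam achievement if undetected.
; After a short delay the game instance loads the next level, with game state depending on whether it is the menu.
; Construction tints a dynamic material orange with a target symbol; pausing disables collision.
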(event EventUnpause
  (Collision|SetActorEnableCollision true))

(event EventPause
  (Collision|SetActorEnableCollision false))

(event EventHitbyPlayer
  (params (HitDirection :type Vector :default "0, 0, 0") (HitLocation :type Vector :default "0, 0, 0") (HitBone :type Name :default "None") (DirectDamage :type Float%20%28single-precision%29) (SpecialDamage :type Special%20Damage%20Struct%20Structure))
  (Utilities|FlowControl|DoOnce false
    (:Completed
      (Components|Animation|PlayAnimation (Variables|Default|GetSkeletalMesh) "/Game/Meshes/Padlock/Animations/Padlock_Anim.Padlock_Anim" false)
      (Physics|SetSimulatePhysics (Variables|Default|GetSkeletalMesh) true)
      (Class|BPICameraFade|FadeOut(Message) (Game|Player|GetPlayerPawn 0))
      (bind _asgi_achery (Utilities|Casting|CastToGI_Achery (Game|GetGameInstance)))
      (Variables|/Game/Blueprints/GI_Achery.GI_Achery_C|SetCurrentGameState _asgi_achery "NewEnumerator3")
      (Default|SaveScore _asgi_achery)
      (Achievment|AchievmentCheckUndetected)
      (Utilities|FlowControl|Delay 1.5)
      (bind _asgi_achery_2 (Utilities|Casting|CastToGI_Achery (Game|GetGameInstance)))
      (Default|LoadLevel _asgi_achery_2 (Variables|Default|GetNewLevel) (select (Utilities|Name|Equal(Name) (Variables|Default|GetNewLevel) "Menu_Environment") "NewEnumerator3" "NewEnumerator0")))))

(fn ConstructionScript
  (bind _mi_padlock (Variables|Default|GetMI_PadLock))
  (CallFunction|CreateMaterialInstance)
  (Rendering|Material|SetTextureParameterValue _mi_padlock "Symbol" "/Game/Textures/HUD/T_Target_A.T_Target_A")
  (Rendering|Material|SetVectorParameterValue _mi_padlock "SymbolColor" "(R=1.000000,G=0.500000,B=0.000000,A=1.000000)" :!class /Script/Engine.MaterialInstanceDynamic)
  (Rendering|Material|SetVectorParameterValue _mi_padlock "PulseColor" "(R=1.000000,G=0.500000,B=0.000000,A=1.000000)" :!class /Script/Engine.MaterialInstanceDynamic)
  (Rendering|Material|SetVectorParameterValue _mi_padlock "BaseColorTint" "(R=1.000000,G=0.500000,B=0.000000,A=1.000000)" :!class /Script/Engine.MaterialInstanceDynamic))

(fn CreateMaterialInstance
  (bind _skeletalmesh (Variables|Default|GetSkeletalMesh))
  (bind _returnvalue (Rendering|Material|CreateDynamicMaterialInstance _skeletalmesh 0 (Rendering|Material|GetMaterial _skeletalmesh 0) "None" :!class /Script/Engine.PrimitiveComponent))
  (Variables|Default|SetMI_PadLock _returnvalue))

(fn AchievmentCheckUndetected
  (if (not (Variables|/Game/Blueprints/VRPawn.VRPawn_C|GetbIsDetected? (.AsVRPawn (Utilities|Casting|CastToVRPawn (Game|Player|GetPlayerPawn 0)))))
    (Default|SetSteamAchievement (.AsBP%20Player%20State (Utilities|Casting|CastToBP_PlayerState (Variables|/Script/Engine.Controller|GetPlayerState (Game|GetPlayerController 0)))) "GENERAL_UNDETECTED")))