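; VR lectern interactable with a book that opens when the VRPawn enters its sphere and closes when it leaves, via IsOpen on AB_Lectern.
; Opening and Closing events play or reverse a timeline that fades book glow, moves and scales an arrow hologram, then loops its animation or hides it with the ribbon effect.
; The construction script creates dynamic materials and sets colors and socket symbol from DamageType.
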(event OnComponentBeginOverlap(Sphere)
  (params (OverlappedComponent :type Primitive%20Component%20Object%20Reference) (OtherActor :type Actor%20Object%20Reference) (OtherComp :type Primitive%20Component%20Object%20Reference) (OtherBodyIndex :type Integer) (bFromSweep :type Boolean) (SweepResult :type Hit%20Result%20Structure%20%28by%20ref%29))
  (Utilities|Casting|CastToVRPawn OtherActor)
  (bind _asab_lectern (Utilities|Casting|CastToAB_Lectern (Components|SkeletalMesh|GetAnimInstance (Variables|Default|GetSkeletalMesh))))
  (Variables|/Game/Meshes/Lectern/Animations/AB_Lectern.AB_Lectern_C|SetisOpen? _asab_lectern true))

(event OnComponentEndOverlap(Sphere)
  (params (OverlappedComponent :type Primitive%20Component%20Object%20Reference) (OtherActor :type Actor%20Object%20Reference) (OtherComp :type Primitive%20Component%20Object%20Reference) (OtherBodyIndex :type Integer))
  (Utilities|Casting|CastToVRPawn OtherActor)
  (bind _asab_lectern (Utilities|Casting|CastToAB_Lectern (Components|SkeletalMesh|GetAnimInstance (Variables|Default|GetSkeletalMesh))))
  (Variables|/Game/Meshes/Lectern/Animations/AB_Lectern.AB_Lectern_C|SetisOpen? _asab_lectern false))

(event Custom|Opening
  (Development|SetHiddeninGame (Variables|Default|GetArrowHologram) false false)
  (Audio|Components|Audio|Play (Variables|Default|GetBookGlowTimer)))

(event Custom|Closing
  (Audio|Components|Audio|Stop (Variables|Default|GetArrowHologram))
  (Utilities|String|Reverse (Variables|Default|GetBookGlowTimer)))

(fn ConstructionScript
  (CallFunction|CreateMaterialInstances)
  (CallFunction|SetColorandSymbol))

(fn CreateMaterialInstances
  (bind _skeletalmesh (Variables|Default|GetSkeletalMesh))
  (bind _skeletalmesh_2 (Variables|Default|GetSkeletalMesh))
  (bind _returnvalue (Rendering|Material|CreateDynamicMaterialInstance _skeletalmesh_2 0 (Rendering|Material|GetMaterial _skeletalmesh_2 0) "None" :!class /Script/Engine.PrimitiveComponent))
  (Variables|Default|SetMI_Book _returnvalue)
  (bind _returnvalue_2 (Rendering|Material|CreateDynamicMaterialInstance _skeletalmesh 1 (Rendering|Material|GetMaterial _skeletalmesh 1) "None" :!class /Script/Engine.PrimitiveComponent))
  (Variables|Default|SetMI_Socket _returnvalue_2))

(fn SetColorandSymbol
  (bind _mi_socket (Variables|Default|GetMI_Socket))
  (bind _damagetype (Variables|Default|GetDamageType))
  (bind _returnvalue (Utilities|Select :Index _damagetype :NewEnumerator8 "(R=1.000000,G=1.000000,B=1.000000,A=1.000000)" :NewEnumerator0 "(R=1.000000,G=0.074631,B=0.000000,A=1.000000)" :NewEnumerator1 "(R=0.000000,G=0.046303,B=0.421875,A=1.000000)" :NewEnumerator2 "(R=0.163719,G=1.000000,B=0.000000,A=1.000000)" :NewEnumerator3 "(R=1.000000,G=1.000000,B=0.200000,A=1.000000)" :NewEnumerator4 "(R=0.642485,G=0.000000,B=1.000000,A=1.000000)" :NewEnumerator5 "(R=0.078125,G=0.019145,B=0.000000,A=1.000000)" :NewEnumerator6 "(R=1.000000,G=0.871168,B=0.000000,A=1.000000)" :NewEnumerator7 "(R=1.000000,G=0.000000,B=0.000000,A=1.000000)"))
  (Rendering|Material|SetVectorParameterValue _mi_socket "G_ChannelColor" _returnvalue :!class /Script/Engine.MaterialInstanceDynamic)
  (Rendering|Material|SetVectorParameterValue _mi_socket "SymbolColor" _returnvalue :!class /Script/Engine.MaterialInstanceDynamic)
  (Rendering|Material|SetVectorParameterValue _mi_socket "DisplayColor" _returnvalue :!class /Script/Engine.MaterialInstanceDynamic)
  (Rendering|Material|SetTextureParameterValue _mi_socket "Symbol" (Utilities|Select :Index (Variables|Default|GetDamageType) :NewEnumerator8 "/Game/Textures/Template/T_Black.T_Black" :NewEnumerator0 "/Game/Textures/MagicSymbols/T_SymbolFire_A.T_SymbolFire_A" :NewEnumerator1 "/Game/Textures/MagicSymbols/T_SymbolIce_A.T_SymbolIce_A" :NewEnumerator2 "/Game/Textures/MagicSymbols/T_SymbolPoison_A.T_SymbolPoison_A" :NewEnumerator3 "/Game/Textures/MagicSymbols/T_SymbolElectricity_A.T_SymbolElectricity_A" :NewEnumerator4 "/Game/Textures/MagicSymbols/T_SymbolGravity_A.T_SymbolGravity_A" :NewEnumerator5 "/Game/Textures/MagicSymbols/T_SymbolExplosion_A.T_SymbolExplosion_A" :NewEnumerator6 "/Game/Textures/MagicSymbols/T_SymbolLuck_A.T_SymbolLuck_A" :NewEnumerator7 "/Game/Textures/MagicSymbols/T_SymbolSuck_A.T_SymbolSuck_A"))
  (Rendering|Material|SetVectorParameterValue (Variables|Default|GetMI_Book) "G_ChannelColor" (* _returnvalue 0.15) :!class /Script/Engine.MaterialInstanceDynamic))