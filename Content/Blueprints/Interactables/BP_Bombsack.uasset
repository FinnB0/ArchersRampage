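; BP_Bombsack is an interactable sack that bursts when the player hits it, spawning bombs.
; A DoOnce on HitbyPlayer hides the intact mesh, reveals the destroyed mesh and turns off actor collision.
; It then spawns a BP_Bomb at each of three spawn-point components and calls GetXP on its experience calculation component.
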(event EventHitbyPlayer
  (params (HitDirection :type Vector :default "0, 0, 0") (HitLocation :type Vector :default "0, 0, 0") (HitBone :type Name :default "None") (DirectDamage :type Float%20%28single-precision%29) (SpecialDamage :type Special%20Damage%20Struct%20Structure))
  (Utilities|FlowControl|DoOnce false
    (:Completed
      (Development|SetHiddeninGame (Variables|Default|GetBombSackMesh) true false)
      (Development|SetHiddeninGame (Variables|Default|GetBombSackMesh_Destroyed) false false)
      (Collision|SetActorEnableCollision false)
      (for _array_element (Utilities|Array|MakeArray (Variables|Default|GetBombSpawn02) (Variables|Default|GetBombSpawn03) (Variables|Default|GetBombSpawn01))
        (Game|SpawnActorfromClass "/Game/Blueprints/Interactables/BP_Bomb.BP_Bomb_C" (Transformation|GetWorldTransform _array_element) "Undefined" 0 0))
      (Default|GetXP (Variables|Default|GetBP_ExperienceCalculationComponent)))))

(fn ConstructionScript)