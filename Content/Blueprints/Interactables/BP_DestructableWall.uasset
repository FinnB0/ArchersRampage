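; BP_DestructableWall is an interactable wall that breaks when hit by one specific special damage type.
; Destruction plays a brick hit sound, activates Niagara effects, swaps the intact mesh for the destroyed one and disables the intact wall's collision.
; It then calls GetXP on its experience component and fires the WallDestroyed dispatcher.
; Pause and Unpause events toggle the actor's collision.
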(event Custom|DestroyWall
  (Audio|PlaySoundatLocation "/Game/Sounds/BrickWall_Hit_Cue.BrickWall_Hit_Cue" (Transformation|GetActorLocation) "0, 0, 0" 1.0 1.0 0.0 0 0 0)
  (Development|SetHiddeninGame (Variables|Default|GetWall_Destroyed) false false)
  (Components|Activation|Activate (Variables|Default|GetNiagara) false)
  (Development|SetHiddeninGame (Variables|Default|GetWall) true false)
  (Collision|SetCollisionEnabled (Variables|Default|GetWall) "NoCollision")
  (Default|GetXP (Variables|Default|GetBP_ExperienceCalculationComponent))
  (Default|CallWallDestroyed))

(event EventUnpause
  (Collision|SetActorEnableCollision true))

(event EventPause
  (Collision|SetActorEnableCollision false))

(event EventBeginPlay
  (Class|NiagaraComponent|SetAsset (Variables|Default|GetNiagara) (Variables|Default|GetNiagaraSystemAsset) true))

(event EventHit
  (params (HitDirection :type Vector :default "0, 0, 0") (HitLocation :type Vector :default "0, 0, 0") (HitBone :type Name :default "None") (DirectDamage :type Float%20%28single-precision%29) (SpecialDamage :type Special%20Damage%20Struct%20Structure) (DamageCauser :type DamageCauserType%20Enum :default "NewEnumerator0"))
  (if (Utilities|Enum|Equal(Enum) (Utilities|Struct|BreakSpecialDamageStruct SpecialDamage) "NewEnumerator5")
    (CallFunction|DestroyWall)))

(fn ConstructionScript)