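; Interactable torch that temporarily goes out when its Hit event fires, then relights itself.
; Hit hides the StaticMesh and Glow components and stops the audio, then restores both components and replays the sound from the start after a short delay.
; The delay is retriggerable, so repeated hits restart the countdown and keep the torch out longer.
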(event EventHit
  (params (HitDirection :type Vector :default "0, 0, 0") (HitLocation :type Vector :default "0, 0, 0") (HitBone :type Name :default "None") (DirectDamage :type Float%20%28single-precision%29) (SpecialDamage :type Special%20Damage%20Struct%20Structure) (DamageCauser :type DamageCauserType%20Enum :default "NewEnumerator0"))
  (Rendering|SetVisibility (Variables|Default|GetStaticMesh) false false)
  (Audio|Components|Audio|Stop (Variables|Default|GetAudio))
  (Utilities|FlowControl|RetriggerableDelay 3.0)
  (Rendering|SetVisibility (Variables|Default|GetStaticMesh) true false)
  (Audio|Components|Audio|Play (Variables|Default|GetAudio) 0.0))

(fn ConstructionScript)