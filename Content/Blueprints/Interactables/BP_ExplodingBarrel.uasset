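; BP_ExplodingBarrel is an interactable barrel that explodes the first time it is hit by the player.
; A DoOnce-guarded HitbyPlayer event plays the explosion sound and spawns a Niagara fire effect whose radius parameter matches the damage radius.
; BPSplashDamageComponent then applies environmental splash damage, BPExperienceCalculationComponent's GetXP is called, and the barrel destroys itself.
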(event EventHitbyPlayer
  (params (HitDirection :type Vector :default "0, 0, 0") (HitLocation :type Vector :default "0, 0, 0") (HitBone :type Name :default "None") (Damage :type Float%20%28single-precision%29) (SpecialDamage :type Special%20Damage%20Struct%20Structure) (bIsEnvironment :type Boolean))
  (bind _returnvalue (Transformation|GetActorLocation))
  (Utilities|FlowControl|DoOnce false
    (:Completed
      (Audio|PlaySoundatLocation "/Game/Sounds/Explosion_Cue.Explosion_Cue" _returnvalue "0, 0, 0" 1.0 1.0 0.0 0 0 0)
      (bind _returnvalue_2 (Niagara|SpawnSystematLocation "/Game/Particles/NS_Barrel_Explode_Fire.NS_Barrel_Explode_Fire" _returnvalue "0, 0, 0" "20.000000,20.000000,20.000000"))
      (Niagara|SetNiagaraVariable(Float) _returnvalue_2 "User.Radius" (Variables|Default|GetDamageRadius))
      (Default|SplashDamage (Variables|Default|GetBP_SplashDamageComponent) (Transformation|GetActorLocation) (Variables|Default|GetDamageRadius) (Variables|Default|GetDefaultDamage) (Variables|Default|GetSpecial%20Damage) true false)
      (Default|GetXP (Variables|Default|GetBP_ExperienceCalculationComponent))
      (Actor|DestroyActor))))

(fn ConstructionScript)