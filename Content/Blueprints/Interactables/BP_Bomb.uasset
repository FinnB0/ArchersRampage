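; BP_Bomb is an interactable explosive that blows up shortly after taking one specific damage type.
; Player hits or applied damage of that type feed a DoOnce, then a short delay destroys the actor.
; Destruction spawns fire explosion effects and sound, deals environmental splash damage of the same type with damage over time, and calls the experience component.
; Pause and Unpause toggle the actor's collision.
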(event EventUnpause
  (Collision|SetActorEnableCollision true))

(event EventPause
  (Collision|SetActorEnableCollision false))

(event EventDestroyed
  (bind _bombmesh (Variables|Default|GetBombMesh))
  (bind _returnvalue (Transformation|GetWorldLocation _bombmesh))
  (Niagara|SpawnSystematLocation "/Game/Particles/NS_Barrel_Explode_Fire.NS_Barrel_Explode_Fire" _returnvalue)
  (Audio|PlaySoundatLocation "/Game/Sounds/Explosion_Cue.Explosion_Cue" _returnvalue "0, 0, 0" 1.0 1.0 0.0 0 0 0)
  (Default|SplashDamage (Variables|Default|GetBP_SplashDamageComponent) (Transformation|GetWorldLocation (Variables|Default|GetBombMesh)) 5e+02 1e+01 (Utilities|Struct|MakeSpecialDamageStruct "NewEnumerator0" 2.0 1e+01 0.1) true)
  (Default|GetXP (Variables|Default|GetBP_ExperienceCalculationComponent)))

(event EventHitbyPlayer
  (params (HitDirection :type Vector :default "0, 0, 0") (HitLocation :type Vector :default "0, 0, 0") (HitBone :type Name :default "None") (DirectDamage :type Float%20%28single-precision%29) (SpecialDamage :type Special%20Damage%20Struct%20Structure))
  (if (Utilities|Enum|Equal(Enum) (Utilities|Struct|BreakSpecialDamageStruct SpecialDamage) "NewEnumerator0")
    (Utilities|FlowControl|DoOnce false
      (:Completed
        (Utilities|FlowControl|Delay 0.5)
        (Actor|DestroyActor)))))

(event EventApplyDamage
  (params (CalculatedDamage :type Float%20%28single-precision%29) (DamageType :type DamageType%20Enum :default "NewEnumerator8"))
  (if (Utilities|Enum|Equal(Enum) DamageType "NewEnumerator0")
    (Utilities|FlowControl|DoOnce false
      (:Completed
        (Utilities|FlowControl|Delay 0.5)
        (Actor|DestroyActor)))))

(fn ConstructionScript)