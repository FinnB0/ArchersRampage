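; Shootable menu button actor that shows either a text symbol or an image in a configurable color.
; The construction script creates dynamic materials for the bloom and image plane, applies color, font, symbol and texture, and uses UsesImage to pick which display is visible in game.
; Taking damage fires the HitButton dispatcher, plays a menu hit sound and plays one of two random hit animations on the skeletal mesh.
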(event EventApplyDamage
  (params (HitDirection :type Vector :default "0, 0, 0") (HitLocation :type Vector :default "0, 0, 0") (HitBone :type Name :default "None") (Damage :type Float%20%28single-precision%29) (DamageType :type DamageType%20Enum :default "NewEnumerator8") (EffectMultiplier :type Float%20%28single-precision%29))
  (Default|CallHitButton)
  (Audio|PlaySoundatLocation "/Game/Sounds/MenuHit_Cue.MenuHit_Cue" (Transformation|GetActorLocation) "0, 0, 0" 1.0 1.0 0.0 0 0 0)
  (Components|Animation|PlayAnimation (Variables|Default|GetSkeletalMesh) (.OutItem (Utilities|Array|Random (Utilities|Array|MakeArray "/Game/Meshes/Buttons/Button01Anim01.Button01Anim01" "/Game/Meshes/Buttons/Button01Anim02.Button01Anim02"))) false))

(fn ConstructionScript
  (bind _textrender (Variables|Default|GetTextRender))
  (bind _imageplane (Variables|Default|GetImagePlane))
  (bind _color (Variables|Default|GetColor))
  (bind _bloom (Variables|Default|GetBloom))
  (bind _returnvalue (Rendering|Material|CreateDynamicMaterialInstance _bloom 0 (Rendering|Material|GetMaterial _bloom 0) "None" :!class /Script/Engine.PrimitiveComponent))
  (Variables|Default|SetM_Bloom _returnvalue)
  (bind _returnvalue_2 (Rendering|Material|CreateDynamicMaterialInstance _imageplane 0 (Rendering|Material|GetMaterial _imageplane 0) "None" :!class /Script/Engine.PrimitiveComponent))
  (Variables|Default|SetMI_Image _returnvalue_2)
  (Class|TextRenderComponent|SetFont (Variables|Default|GetTextRender) (Variables|Default|GetFont))
  (Rendering|Components|TextRender|SetText _textrender (Variables|Default|GetSymbol))
  (Rendering|Components|TextRender|SetTextRenderColor _textrender (Math|Conversions|ToColor(LinearColor) _color false))
  (Rendering|Material|SetVectorParameterValue (Variables|Default|GetM_Bloom) "EmissiveColor" _color :!class /Script/Engine.MaterialInstanceDynamic)
  (Rendering|Material|SetVectorParameterValue (Variables|Default|GetMI_Image) "BaseColorTint" _color :!class /Script/Engine.MaterialInstanceDynamic)
  (Rendering|Material|SetTextureParameterValue (Variables|Default|GetMI_Image) "OpacityMap" (Variables|Default|GetImage))
  (if (Variables|Default|GetbUsesImage?)
    (Development|SetHiddeninGame (Variables|Default|GetImagePlane) false false)
    (Development|SetHiddeninGame (Variables|Default|GetTextRender) true false)
    (else
      (Development|SetHiddeninGame (Variables|Default|GetImagePlane) true false)
      (Development|SetHiddeninGame (Variables|Default|GetTextRender) false false))))